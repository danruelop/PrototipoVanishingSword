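; Shared two-player camera that both controllers blend to shortly after BeginPlay.
; Each Tick it centers on the pawns' midpoint and scales spring arm length by their 2D or 3D distance, within height limits.
; At maximum zoom it projects pawns to screen and, at top or left margins, nudges either pawn inward in camera-yaw space, depending on which is moving.
; The left margin varies with screen height; only these two edges are tested.
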(event EventBeginPlay
  (Utilities|FlowControl|Delay 0.2)
  (Game|Player|SetViewTargetwithBlend (Game|GetPlayerController 0) self 1.0 "VTBlend_Linear" 0.0 false)
  (Utilities|FlowControl|Delay 1.0)
  (Variables|Default|SetCameraSetted true)
  (Variables|Default|SetSpringArmRotationZ (.yaw (Class|SpringArmComponent|GetTargetRotation (Variables|Default|GetSpringArm)))))

(event EventTick
  (params (DeltaSeconds :type Float%20%28single-precision%29))
  (bind _returnvalue (Game|Player|GetPlayerPawn 1))
  (bind _returnvalue_2 (Game|GetPlayerController 0))
  (bind _returnvalue_3 (Game|Player|GetPlayerPawn 1))
  (bind _returnvalue_4 (Game|Player|GetPlayerPawn 1))
  (bind _returnvalue_5 (Game|Player|GetPlayerPawn 0))
  (bind _returnvalue_6 (Game|GetPlayerController 0))
  (bind _returnvalue_7 (Game|Player|GetPlayerPawn 0))
  (bind _returnvalue_8 (Game|Player|GetPlayerPawn 0))
  (bind _returnvalue_9 (Game|Player|GetPlayerPawn 1))
  (bind _returnvalue_10 (Game|Player|GetPlayerPawn 0))
  (bind _returnvalue_11 (Game|GetPlayerController 0))
  (bind _returnvalue_12 (Game|Player|GetPlayerPawn 1))
  (bind _returnvalue_13 (Game|GetPlayerController 0))
  (bind _returnvalue_14 (Game|Player|GetPlayerPawn 0))
  (bind _returnvalue_15 (Game|Player|GetPlayerPawn 1))
  (bind _returnvalue_16 (Viewport|GetViewportSize))
  (bind _returnvalue_17 (Game|Player|GetPlayerPawn 0))
  (bind _returnvalue_18 (Game|GetPlayerController 0))
  (bind _returnvalue_19 (Game|GetPlayerController 0))
  (bind _returnvalue_20 (Game|Player|GetPlayerPawn 0))
  (bind _returnvalue_21 (Game|Player|GetPlayerPawn 1))
  (bind _returnvalue_22 (Viewport|GetViewportSize))
  (bind _topgapedge (Variables|Default|GetTopGapEdge))
  (bind _extrasidesedge (Variables|Default|GetExtraSidesEdge))
  (bind _leftgapedge (Variables|Default|GetLeftGapEdge))
  (bind _extrasidesedge_2 (Variables|Default|GetExtraSidesEdge))
  (bind _topgapedge_2 (Variables|Default|GetTopGapEdge))
  (bind _topgapedge_3 (Variables|Default|GetTopGapEdge))
  (bind _topgapedge_4 (Variables|Default|GetTopGapEdge))
  (bind _leftgapedge_2 (Variables|Default|GetLeftGapEdge))
  (bind _springarmrotationz (Variables|Default|GetSpringArmRotationZ))
  (bind _springarmrotationz_2 (Variables|Default|GetSpringArmRotationZ))
  (bind _springarmrotationz_3 (Variables|Default|GetSpringArmRotationZ))
  (bind _springarmrotationz_4 (Variables|Default|GetSpringArmRotationZ))
  (bind _springarmrotationz_5 (Variables|Default|GetSpringArmRotationZ))
  (bind _springarmrotationz_6 (Variables|Default|GetSpringArmRotationZ))
  (bind _springarmrotationz_7 (Variables|Default|GetSpringArmRotationZ))
  (bind _springarmrotationz_8 (Variables|Default|GetSpringArmRotationZ))
  (bind _springarmrotationz_9 (Variables|Default|GetSpringArmRotationZ))
  (bind _returnvalue_23 (Transformation|GetActorLocation _returnvalue))
  (bind _returnvalue_24 (Transformation|GetActorLocation _returnvalue_3))
  (bind _returnvalue_25 (Transformation|GetActorLocation _returnvalue_4))
  (bind _returnvalue_26 (Transformation|GetActorLocation _returnvalue_5))
  (bind _returnvalue_27 (Transformation|GetVelocity _returnvalue_4))
  (bind _returnvalue_28 (Transformation|GetActorLocation _returnvalue_7))
  (bind _returnvalue_29 (Transformation|GetActorLocation _returnvalue_8))
  (bind _returnvalue_30 (Transformation|GetVelocity _returnvalue_7))
  (bind _returnvalue_31 (Transformation|GetActorLocation _returnvalue_9))
  (bind _returnvalue_32 (Transformation|GetActorLocation _returnvalue_10))
  (bind _returnvalue_33 (Transformation|GetActorLocation _returnvalue_12))
  (bind _returnvalue_34 (Transformation|GetActorLocation _returnvalue_14))
  (bind _returnvalue_35 (Transformation|GetActorLocation _returnvalue_15))
  (bind _returnvalue_36 (Transformation|GetVelocity _returnvalue_15))
  (bind _returnvalue_37 (- (.y _returnvalue_16) _topgapedge_2))
  (bind _returnvalue_38 (Transformation|GetActorLocation _returnvalue_17))
  (bind _returnvalue_39 (Transformation|GetActorLocation _returnvalue_20))
  (bind _returnvalue_40 (Transformation|GetVelocity _returnvalue_20))
  (bind _returnvalue_41 (Transformation|GetActorLocation _returnvalue_21))
  (bind _returnvalue_42 (- (.y _returnvalue_22) _topgapedge_3))
  (bind _returnvalue_43 (* _springarmrotationz_2 -1.0))
  (bind _returnvalue_44 (* _springarmrotationz_3 -1.0))
  (bind _returnvalue_45 (* _springarmrotationz_4 -1.0))
  (bind _returnvalue_46 (* _springarmrotationz_5 -1.0))
  (bind _returnvalue_47 (* _springarmrotationz_6 -1.0))
  (bind _returnvalue_48 (* _springarmrotationz_7 -1.0))
  (bind _returnvalue_49 (* _springarmrotationz_8 -1.0))
  (bind _returnvalue_50 (* _springarmrotationz_9 -1.0))
  (bind _screenposition (Class|GameplayStatics|ProjectWorldtoScreen _returnvalue_2 _returnvalue_24 false))
  (bind _returnvalue_51 (Math|Vector|RotateVector _returnvalue_25 (Math|Rotator|MakeRotator 0.0 0.0 _returnvalue_45)))
  (bind _returnvalue_52 (Math|Vector|RotateVector _returnvalue_26 (Math|Rotator|MakeRotator 0.0 0.0 _returnvalue_46)))
  (bind _returnvalue_53 (Math|Vector|RotateVector _returnvalue_28 (Math|Rotator|MakeRotator 0.0 0.0 _returnvalue_47)))
  (bind _returnvalue_54 (Math|Vector|RotateVector _returnvalue_31 (Math|Rotator|MakeRotator 0.0 0.0 _returnvalue_48)))
  (bind _returnvalue_55 (Math|Vector|RotateVector _returnvalue_32 (Math|Rotator|MakeRotator 0.0 0.0 _returnvalue_49)))
  (bind _screenposition_2 (Class|GameplayStatics|ProjectWorldtoScreen _returnvalue_11 _returnvalue_33 false))
  (bind _screenposition_3 (Class|GameplayStatics|ProjectWorldtoScreen _returnvalue_13 _returnvalue_34 false))
  (bind _returnvalue_56 (Math|Vector|RotateVector _returnvalue_35 (Math|Rotator|MakeRotator 0.0 0.0 _returnvalue_50)))
  (bind _screenposition_4 (Class|GameplayStatics|ProjectWorldtoScreen _returnvalue_18 _returnvalue_38 false))
  (bind _returnvalue_57 (Math|Vector|RotateVector _returnvalue_39 (Math|Rotator|MakeRotator 0.0 0.0 _returnvalue_43)))
  (bind _returnvalue_58 (Math|Vector|RotateVector _returnvalue_40 (Math|Rotator|MakeRotator 0.0 0.0 _springarmrotationz)))
  (bind _returnvalue_59 (Math|Vector|RotateVector _returnvalue_41 (Math|Rotator|MakeRotator 0.0 0.0 _returnvalue_44)))
  (bind _returnvalue_60 (- _returnvalue_29 _returnvalue_23))
  (bind _returnvalue_61 (Math|Float|MapRangeClamped (.y _screenposition_2) _topgapedge_2 _returnvalue_37 0.0 1.0))
  (bind _returnvalue_62 (Math|Float|MapRangeClamped (.y _screenposition_3) _topgapedge_3 _returnvalue_42 0.0 1.0))
  (bind _returnvalue_63 (- 1.0 _returnvalue_61))
  (bind _returnvalue_64 (- 1.0 _returnvalue_62))
  (bind _returnvalue_65 (* _returnvalue_63 _extrasidesedge))
  (bind _returnvalue_66 (* _returnvalue_64 _extrasidesedge_2))
  (bind _returnvalue_67 (+ _leftgapedge_2 _returnvalue_65))
  (bind _returnvalue_68 (+ _leftgapedge _returnvalue_66))
  ;[1 1 1] Zoom and movement between players
  (if (Variables|Default|GetDistance2D)
    (Variables|Default|SetDistanceVectorLength (Math|Vector2D|Vector2DLength (- (Math|Conversions|ToVector2D(Vector) _returnvalue_29) (Math|Conversions|ToVector2D(Vector) _returnvalue_23))))
    (else
      (Variables|Default|SetDistanceVectorLength (Math|Vector|VectorLength _returnvalue_60))))
  (Transformation|SetActorLocation (+ _returnvalue_23 (/ _returnvalue_60 2.0)) false false)
  (Variables|/Script/Engine.SpringArmComponent|SetTargetArmLength (Variables|Default|GetSpringArm) (Math|Float|Clamp(Float) (* (Variables|Default|GetDistanceVectorLength) (Variables|Default|GetMultiplierDistanceHeight)) (Variables|Default|GetMinHeight) (Variables|Default|GetMaxHeight)))
  (if (Variables|Default|GetCameraSetted)
    (if (== (Math|Float|Clamp(Float) (* (Variables|Default|GetDistanceVectorLength) (Variables|Default|GetMultiplierDistanceHeight)) (Variables|Default|GetMinHeight) (Variables|Default|GetMaxHeight)) (Variables|Default|GetMaxHeight))
      ;[1 1 1] TOP EDGE - Player 0
      (if (<= (.y (.ScreenPosition (Class|GameplayStatics|ProjectWorldtoScreen _returnvalue_19 (Transformation|GetActorLocation (Game|Player|GetPlayerPawn 0)) false))) (.y (.ScreenPosition (Class|GameplayStatics|ProjectWorldtoScreen _returnvalue_19 (Transformation|GetActorLocation (Game|Player|GetPlayerPawn 1)) false))))
        (if (and (< (.y _screenposition_4) (+ _topgapedge_4 3.0)) (> (.y _screenposition_4) _topgapedge_4))
          _
          (elif (<= (.y _screenposition_4) (Variables|Default|GetTopGapEdge))
            (if (== (.X (Math|Vector|BreakVector _returnvalue_58)) 0.0)
              (Transformation|SetActorLocation _returnvalue_21 (Math|Vector|RotateVector (Math|Vector|MakeVector (+ (* DeltaSeconds (Math|Vector|VectorLength (Transformation|GetVelocity _returnvalue_21))) (.x _returnvalue_59)) (.y _returnvalue_59) (.z _returnvalue_59)) (Math|Rotator|MakeRotator 0.0 0.0 (Variables|Default|GetSpringArmRotationZ))) false false)
              (else
                (Transformation|SetActorLocation _returnvalue_20 (Math|Vector|RotateVector (Math|Vector|MakeVector (- (.x _returnvalue_57) (* DeltaSeconds (Math|Vector|VectorLength _returnvalue_58))) (.y _returnvalue_57) (.z _returnvalue_57)) (Math|Rotator|MakeRotator 0.0 0.0 (Variables|Default|GetSpringArmRotationZ))) false false)))))
        (else
          ;[1 1 1] TOP EDGE - Player 1
          (if (and (< (.y _screenposition) (+ _topgapedge 3.0)) (> (.y _screenposition) _topgapedge))
            _
            (elif (<= (.y _screenposition) (Variables|Default|GetTopGapEdge))
              (if (Math|Vector|Equal(Vector) _returnvalue_27 "0, 0, 0" 0.0001)
                (Transformation|SetActorLocation _returnvalue_5 (Math|Vector|RotateVector (Math|Vector|MakeVector (+ (* DeltaSeconds (Math|Vector|VectorLength (Transformation|GetVelocity _returnvalue_5))) (.x _returnvalue_52)) (.y _returnvalue_52) (.z _returnvalue_52)) (Math|Rotator|MakeRotator 0.0 0.0 (Variables|Default|GetSpringArmRotationZ))) false false)
                (else
                  (Transformation|SetActorLocation _returnvalue_4 (Math|Vector|RotateVector (Math|Vector|MakeVector (- (.x _returnvalue_51) (* DeltaSeconds (Math|Vector|VectorLength _returnvalue_27))) (.y _returnvalue_51) (.z _returnvalue_51)) (Math|Rotator|MakeRotator 0.0 0.0 (Variables|Default|GetSpringArmRotationZ))) false false)))))))
      ;[1 1 1] LEFT EDGE - Player 0
      (if (<= (.x (.ScreenPosition (Class|GameplayStatics|ProjectWorldtoScreen _returnvalue_6 (Transformation|GetActorLocation (Game|Player|GetPlayerPawn 0)) false))) (.x (.ScreenPosition (Class|GameplayStatics|ProjectWorldtoScreen _returnvalue_6 (Transformation|GetActorLocation (Game|Player|GetPlayerPawn 1)) false))))
        (if (not (and (< (.x _screenposition_3) (+ _returnvalue_68 3.0)) (> (.x _screenposition_3) _returnvalue_68)))
          (if (<= (.x _screenposition_3) _returnvalue_68)
            (if (== (.Y (Math|Vector|BreakVector (Math|Vector|RotateVector _returnvalue_30 (Math|Rotator|MakeRotator 0.0 0.0 (Variables|Default|GetSpringArmRotationZ))))) 0.0)
              (Transformation|SetActorLocation _returnvalue_9 (Math|Vector|RotateVector (Math|Vector|MakeVector (.x _returnvalue_54) (- (.y _returnvalue_54) (* DeltaSeconds (Math|Vector|VectorLength (Transformation|GetVelocity _returnvalue_9)))) (.z _returnvalue_54)) (Math|Rotator|MakeRotator 0.0 0.0 (Variables|Default|GetSpringArmRotationZ))) false false)
              (else
                (Transformation|SetActorLocation _returnvalue_7 (Math|Vector|RotateVector (Math|Vector|MakeVector (.x _returnvalue_53) (+ (* DeltaSeconds (Math|Vector|VectorLength _returnvalue_30)) (.y _returnvalue_53)) (.z _returnvalue_53)) (Math|Rotator|MakeRotator 0.0 0.0 (Variables|Default|GetSpringArmRotationZ))) false false)))))
        (else
          ;[1 1 1] LEFT EDGE - Player 1
          (if (not (and (< (.x _screenposition_2) (+ _returnvalue_67 3.0)) (> (.x _screenposition_2) _returnvalue_67)))
            (if (<= (.x _screenposition_2) _returnvalue_67)
              (if (== (.y (Math|Vector|RotateVector _returnvalue_36 (Math|Rotator|MakeRotator 0.0 0.0 (Variables|Default|GetSpringArmRotationZ)))) 0.0)
                (Transformation|SetActorLocation _returnvalue_10 (Math|Vector|RotateVector (Math|Vector|MakeVector (.x _returnvalue_55) (- (.y _returnvalue_55) (* DeltaSeconds (Math|Vector|VectorLength (Transformation|GetVelocity _returnvalue_10)))) (.z _returnvalue_55)) (Math|Rotator|MakeRotator 0.0 0.0 (Variables|Default|GetSpringArmRotationZ))) false false)
                (else
                  (Transformation|SetActorLocation _returnvalue_15 (Math|Vector|RotateVector (Math|Vector|MakeVector (.x _returnvalue_56) (+ (* DeltaSeconds (Math|Vector|VectorLength _returnvalue_36)) (.y _returnvalue_56)) (.z _returnvalue_56)) (Math|Rotator|MakeRotator 0.0 0.0 (Variables|Default|GetSpringArmRotationZ))) false false))))))))))

(fn ConstructionScript)