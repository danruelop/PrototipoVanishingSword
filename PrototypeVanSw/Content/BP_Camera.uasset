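; Shared camera for two local players that follows their midpoint and keeps them from leaving the top and bottom of the screen.
; Each tick it scales the spring arm length from the players' distance, clamped between height limits.
; After the startup view blend, screen-edge deprojection and line traces place top and bottom collision walls, enabled when either player nears that edge.
; An older max-zoom wall version remains unused.
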(event EventBeginPlay
  (Utilities|FlowControl|Delay 0.2)
  (Game|Player|SetViewTargetwithBlend (Game|GetPlayerController 0) self 1.0 "VTBlend_Linear" 0.0 false)
  (Utilities|FlowControl|Delay 1.0)
  (Variables|Default|SetCameraSetted true))

(event EventTick
  (params (DeltaSeconds :type Float%20%28single-precision%29))
  (bind _returnvalue (Game|Player|GetPlayerPawn 1))
  (bind _returnvalue_2 (Game|GetPlayerController 0))
  (bind _returnvalue_3 (Game|GetPlayerController 0))
  (bind _returnvalue_4 (Game|Player|GetPlayerPawn 0))
  (bind _boxbottom (Variables|Default|GetBoxBottom))
  (bind _boxtop (Variables|Default|GetBoxTop))
  (bind _boxtop_2 (Variables|Default|GetBoxTop))
  (bind _boxtop_3 (Variables|Default|GetBoxTop))
  (bind _boxbottom_2 (Variables|Default|GetBoxBottom))
  (bind _boxbottom_3 (Variables|Default|GetBoxBottom))
  (bind _returnvalue_5 (Transformation|GetActorLocation _returnvalue))
  (bind _returnvalue_6 (Transformation|GetActorLocation _returnvalue_4))
  (bind _returnvalue_7 (- _returnvalue_6 _returnvalue_5))
  ;[1 1 1] Zoom and movement between players
  (if (Variables|Default|GetDistance2D)
    (Variables|Default|SetDistanceVectorLength (Math|Vector2D|Vector2DLength (- (Math|Conversions|ToVector2D(Vector) _returnvalue_6) (Math|Conversions|ToVector2D(Vector) _returnvalue_5))))
    (else
      (Variables|Default|SetDistanceVectorLength (Math|Vector|VectorLength _returnvalue_7))))
  (Transformation|SetActorLocation (+ _returnvalue_5 (/ _returnvalue_7 2.0)) false false)
  (Variables|/Script/Engine.SpringArmComponent|SetTargetArmLength (Variables|Default|GetSpringArm) (Math|Float|Clamp(Float) (* (Variables|Default|GetDistanceVectorLength) (Variables|Default|GetMultiplierDistanceHeight)) (Variables|Default|GetMinHeight) (Variables|Default|GetMaxHeight)))
  (if (Variables|Default|GetCameraSetted)
    ;[1 1 1] Top wall setup
    (if (<= (.y (.ScreenPosition (Class|GameplayStatics|ProjectWorldtoScreen _returnvalue_3 (Transformation|GetActorLocation (Game|Player|GetPlayerPawn 0)) false))) (.y (.ScreenPosition (Class|GameplayStatics|ProjectWorldtoScreen _returnvalue_3 (Transformation|GetActorLocation (Game|Player|GetPlayerPawn 1)) false))))
      (Variables|Default|SetScreenPositionXTop (.x (.ScreenPosition (Class|GameplayStatics|ProjectWorldtoScreen (Game|GetPlayerController 0) (Transformation|GetActorLocation (Game|Player|GetPlayerPawn 0)) false))))
      (else
        (Variables|Default|SetScreenPositionXTop (.x (.ScreenPosition (Class|GameplayStatics|ProjectWorldtoScreen (Game|GetPlayerController 0) (Transformation|GetActorLocation (Game|Player|GetPlayerPawn 1)) false))))))
    (bind _outhit (Collision|LineTraceByChannel (.WorldPosition (Class|GameplayStatics|DeprojectScreentoWorld (Game|GetPlayerController 0) (Math|Vector2D|MakeVector2D (Variables|Default|GetScreenPositionXTop) 1e+02))) (+ (.WorldPosition (Class|GameplayStatics|DeprojectScreentoWorld (Game|GetPlayerController 0) (Math|Vector2D|MakeVector2D (Variables|Default|GetScreenPositionXTop) 1e+02))) (* (.WorldDirection (Class|GameplayStatics|DeprojectScreentoWorld (Game|GetPlayerController 0) (Math|Vector2D|MakeVector2D (Variables|Default|GetScreenPositionXTop) 1e+02))) (* (Variables|Default|GetMaxHeight) 2.0))) "TraceTypeQuery1" false 0 "ForOneFrame"))
    (if (or (>= (+ (.x (Transformation|GetActorLocation (Game|Player|GetPlayerPawn 0))) 175.0) (.X (Math|Vector|BreakVector (.location _outhit)))) (>= (+ (.x (Transformation|GetActorLocation (Game|Player|GetPlayerPawn 1))) 175.0) (.X (Math|Vector|BreakVector (.location _outhit)))))
      (Transformation|SetWorldLocation _boxtop (.location _outhit) false false)
      (Transformation|SetWorldScale3D _boxtop (Math|Vector|MakeVector 1.0 1e+02 1e+01))
      (Collision|SetCollisionEnabled _boxtop_3 "QueryAndPhysics")
      (Collision|SetCollisionEnabled (Variables|Default|GetCubeTop) "QueryAndPhysics")
      (Rendering|SetVisibility _boxtop_3 true true)
      (else
        (Collision|SetCollisionEnabled _boxtop_2 "NoCollision")
        (Collision|SetCollisionEnabled (Variables|Default|GetCubeTop) "NoCollision")
        (Rendering|SetVisibility _boxtop_2 false true)))
    ;[1 1 1] Bottom wall setup
    (if (>= (.y (.ScreenPosition (Class|GameplayStatics|ProjectWorldtoScreen _returnvalue_2 (Transformation|GetActorLocation (Game|Player|GetPlayerPawn 0)) false))) (.y (.ScreenPosition (Class|GameplayStatics|ProjectWorldtoScreen _returnvalue_2 (Transformation|GetActorLocation (Game|Player|GetPlayerPawn 1)) false))))
      (Variables|Default|SetScreenPositionXBottom (.x (.ScreenPosition (Class|GameplayStatics|ProjectWorldtoScreen (Game|GetPlayerController 0) (Transformation|GetActorLocation (Game|Player|GetPlayerPawn 0)) false))))
      (else
        (Variables|Default|SetScreenPositionXBottom (.x (.ScreenPosition (Class|GameplayStatics|ProjectWorldtoScreen (Game|GetPlayerController 0) (Transformation|GetActorLocation (Game|Player|GetPlayerPawn 1)) false))))))
    (bind _outhit_2 (Collision|LineTraceByChannel (.WorldPosition (Class|GameplayStatics|DeprojectScreentoWorld (Game|GetPlayerController 0) (Math|Vector2D|MakeVector2D (Variables|Default|GetScreenPositionXBottom) (- (.y (Viewport|GetViewportSize)) 3e+01)))) (+ (.WorldPosition (Class|GameplayStatics|DeprojectScreentoWorld (Game|GetPlayerController 0) (Math|Vector2D|MakeVector2D (Variables|Default|GetScreenPositionXBottom) (- (.y (Viewport|GetViewportSize)) 3e+01)))) (* (.WorldDirection (Class|GameplayStatics|DeprojectScreentoWorld (Game|GetPlayerController 0) (Math|Vector2D|MakeVector2D (Variables|Default|GetScreenPositionXBottom) (- (.y (Viewport|GetViewportSize)) 3e+01)))) (* (Variables|Default|GetMaxHeight) 2.0))) "TraceTypeQuery1" false 0 "ForOneFrame"))
    (if (or (<= (+ (.x (Transformation|GetActorLocation (Game|Player|GetPlayerPawn 0))) -175.0) (.X (Math|Vector|BreakVector (.location _outhit_2)))) (<= (+ (.x (Transformation|GetActorLocation (Game|Player|GetPlayerPawn 1))) -175.0) (.X (Math|Vector|BreakVector (.location _outhit_2)))))
      (Transformation|SetWorldLocation _boxbottom (.location _outhit_2) false false)
      (Transformation|SetWorldScale3D _boxbottom (Math|Vector|MakeVector 1.0 1e+02 1e+01))
      (Components|Box|SetBoxExtent _boxbottom (.BoxExtent (Collision|GetComponentBounds (Variables|Default|GetCubeBottom))) true)
      (Collision|SetCollisionEnabled _boxbottom_2 "QueryAndPhysics")
      (Collision|SetCollisionEnabled (Variables|Default|GetCubeBottom) "QueryAndPhysics")
      (Rendering|SetVisibility _boxbottom_2 true true)
      (else
        (Collision|SetCollisionEnabled _boxbottom_3 "NoCollision")
        (Collision|SetCollisionEnabled (Variables|Default|GetCubeBottom) "NoCollision")
        (Rendering|SetVisibility _boxbottom_3 false true)))))

(fn ConstructionScript)