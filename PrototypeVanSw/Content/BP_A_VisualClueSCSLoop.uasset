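; BP_A_VisualClueSCSLoop is a short-lived visual clue actor that makes five sphere components rise through the world.
; BeginPlay gathers the preplaced sphere components into the AllSpheres array, then destroys the actor after LifeTime.
; Each Tick loops over that array, raising each sphere's world Z by UpVelocityPerSecond scaled by delta time, so motion is frame-rate independent.
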(event EventBeginPlay
  (Utilities|FlowControl|Sequence
    (:then_0
      (CallFunction|PopulateAllSpheres))
    (:then_1
      (Utilities|FlowControl|Delay (Variables|Default|GetlifeTime))
      (Actor|DestroyActor))))

(event Collision|EventActorBeginOverlap
  (params (OtherActor :type Actor%20Object%20Reference)))

(event EventTick
  (params (DeltaSeconds :type Float%20%28single-precision%29))
  (CallFunction|Move DeltaSeconds))

(fn ConstructionScript)

(fn Move
  (params (deltaSeconds :type Float%20%28single-precision%29))
  (for _array_element (Variables|Default|GetallSpheres)
    (Transformation|SetWorldLocation _array_element (Math|Vector|MakeVector (.x (Transformation|GetWorldLocation _array_element)) (.y (Transformation|GetWorldLocation _array_element)) (+ (.z (Transformation|GetWorldLocation _array_element)) (* deltaSeconds (Variables|Default|GetupVelocityPerSecond)))) false false)))

(fn PopulateAllSpheres
  (Utilities|FlowControl|Sequence
    (:then_0
      (Utilities|Array|Add (Variables|Default|GetallSpheres) (Variables|Default|GetSphere)))
    (:then_1
      (Utilities|Array|Add (Variables|Default|GetallSpheres) (Variables|Default|GetSphere1)))
    (:then_2
      (Utilities|Array|Add (Variables|Default|GetallSpheres) (Variables|Default|GetSphere2)))
    (:then_3
      (Utilities|Array|Add (Variables|Default|GetallSpheres) (Variables|Default|GetSphere3)))
    (:then_4
      (Utilities|Array|Add (Variables|Default|GetallSpheres) (Variables|Default|GetSphere4)))))