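; Player character that plays either a sword-wielding, corruption-marked DPS or a stunning Support, swapping roles with other players via the sword.
; As Support, holding TakeSword detaches the sword and times the press for a trace on release.
; When the trace finishes, a SwitchSword dispatcher bound across all BP_Players flips every role, and the UI is notified.
; Attack and stun briefly enable overlap zones that send damage or stun messages, with movement locks and timer cooldowns.
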(event OnComponentBeginOverlap(DPS_AttackZone)
  (params (OverlappedComponent :type Primitive%20Component%20Object%20Reference) (OtherActor :type Actor%20Object%20Reference) (OtherComp :type Primitive%20Component%20Object%20Reference) (OtherBodyIndex :type Integer) (bFromSweep :type Boolean) (SweepResult :type Hit%20Result%20Structure%20%28by%20ref%29))
  (Class|BPIonHit|ApplyDamage(Message) OtherActor (Variables|Default|GetiDPSBasicAttackDamage)))

(event OnComponentBeginOverlap(SUPP_StunZone)
  (params (OverlappedComponent :type Primitive%20Component%20Object%20Reference) (OtherActor :type Actor%20Object%20Reference) (OtherComp :type Primitive%20Component%20Object%20Reference) (OtherBodyIndex :type Integer) (bFromSweep :type Boolean) (SweepResult :type Hit%20Result%20Structure%20%28by%20ref%29))
  (Class|BPIonHit|ApplyStun(Message) OtherActor))

(event Custom|Event%20TakeSword
  ;[1 1 1] All Players have to "listen" to Switch Sword event in case it is activated
  (if (Rendering|IsVisible (Variables|Default|GetCorruptionCircleVFX))
    (Rendering|SetVisibility (Variables|Default|GetCorruptionCircleVFX) false false))
  (bind _output_get (Variables|Default|SetbIsDPS (not (Variables|Default|GetbIsDPS))))
  (if _output_get
    (CallFunction|ClaimSword)
    (Rendering|SetVisibility (Variables|Default|GetCorruptionVFX) true false)
    (else
      ;[1 1 1] Deactivate attack zone from the other player
      (CallFunction|DeactivateZone (Variables|Default|GetDPS_AttackZone))
      (Rendering|SetVisibility (Variables|Default|GetCorruptionVFX) false false))))

(event Custom|finishedhittingTakeSword
  (bind _returnvalue (Actor|GetActorOfClass "/Game/UI/UI_Code/BP_UI_Master.BP_UI_Master_C"))
  (Class|BPIonHit|SetPlayerAffectedbyCorruption(Message) _returnvalue (Variables|Default|GetiPlayerIndex))
  (Default|CallSwitchSword)
  (|CollapseGraph_0 (Variables|Default|GetblsTakeSword) 0.37))

(event EventBeginPlay
  (Rendering|SetVisibility (Variables|Default|GetCorruptionVFX) (Variables|Default|GetbIsDPS) false)
  ;[1 1 1] All Players have to "listen" to Switch Sword event in case it is activated
  (EventDispatchers|BindEventtoHittingFinished (Variables|Default|GettakeSwordTrace) (delegate Custom|finishedhittingTakeSword))
  (Utilities|FlowControl|Sequence
    (:then_0
      (bind _outactors (Actor|GetAllActorsOfClass "BP_Player_C"))
      (for _array_element _outactors
        (EventDispatchers|BindEventtoSwitchSword _array_element (delegate Custom|Event%20TakeSword))))
    (:then_1
      (CallFunction|DeactivateZone (Variables|Default|GetDPS_AttackZone))
      (CallFunction|DeactivateZone (Variables|Default|GetSUPP_StunZone)))))

(event Collision|EventActorBeginOverlap
  (params (OtherActor :type Actor%20Object%20Reference)))

(event EventTick
  (params (DeltaSeconds :type Float%20%28single-precision%29))
  (if (Variables|Default|GetPressed)
    (Variables|Default|SetTimePress (+ DeltaSeconds (Variables|Default|GetTimePress)))))

(event Input|ActionEvents|InputActionBasicAttack/Stun
  (params (Key :type Key%20Structure :default "None"))
  (:Pressed
    (if (Variables|Default|GetbIsDPS)
      (|DPSAttack)
      (else
        (|SUPPStun)))))

(event Input|ActionEvents|InputActionTakeSword
  (params (Key :type Key%20Structure :default "None"))
  (bind _charactermovement (Variables|Character|GetCharacterMovement))
  ;[1 1 1] Player receives TakeSword input and call Switch Sword event
  (:Pressed
    (if (not (Variables|Default|GetbIsDPS))
      (Variables|Default|SetTimePress 0.0)
      (Variables|Default|SetPressed true)
      (CallFunction|UnClaimSword)
      (Pawn|Components|CharacterMovement|DisableMovement _charactermovement)
      (Components|Movement|StopMovementImmediately _charactermovement)))
  (:Released
    (Variables|Default|SetPressed false)
    (if (not (Variables|Default|GetbIsDPS))
      (Default|TraceTakeSword (Variables|Default|GettakeSwordTrace) (Variables|Default|GetTimePress))
      (Pawn|Components|CharacterMovement|SetMovementMode _charactermovement "MOVE_Walking" 0))))

(event Input|ActionEvents|InputActionPauseMenu
  (params (Key :type Key%20Structure :default "None"))
  (:Pressed
    (bind _returnvalue (Actor|GetActorOfClass "/Game/UI/UI_Code/BP_UI_Master.BP_UI_Master_C"))
    (Class|BPIonHit|OpenPauseMenu(Message) _returnvalue)))

(fn ConstructionScript)

(fn ClaimSword
  (bind _returnvalue (Actor|GetActorOfClass "/Game/Code/Player/BP_Sword.BP_Sword_C"))
  (Transformation|AttachComponentToComponent _returnvalue (Variables|Default|GetSword) "SwordSocket" "SnapToTarget" "SnapToTarget" "KeepWorld" true))

(fn StartDPSAttackCooldown
  (Variables|Default|SetbIsDPSAttackInCooldown false))

(fn StartSUPPStunCooldown
  (Variables|Default|SetbIsSUPPStunInCooldown false))

(fn ActivateZone
  (params (Zone%20Ref :type Static%20Mesh%20Component%20Object%20Reference))
  (Components|Activation|SetActive Zone%20Ref true false)
  (Rendering|SetVisibility Zone%20Ref true false)
  (Collision|SetCollisionEnabled Zone%20Ref "QueryOnly"))

(fn DeactivateZone
  (params (Zone%20Ref :type Static%20Mesh%20Component%20Object%20Reference))
  (Components|Activation|SetActive Zone%20Ref false false)
  (Rendering|SetVisibility Zone%20Ref false false)
  (Collision|SetCollisionEnabled Zone%20Ref "NoCollision"))

(fn UnClaimSword
  (bind _returnvalue (Actor|GetActorOfClass "/Game/Code/Player/BP_Sword.BP_Sword_C"))
  (Transformation|DetachFromActor _returnvalue "KeepWorld" "KeepWorld" "KeepWorld")
  (Transformation|SetActorLocation _returnvalue "0, 0,-100.000000" false false))

(fn ActivateCorruptionCircleVFX
  (Rendering|SetVisibility (Variables|Default|GetCorruptionCircleVFX) true false))