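; BP_C_MarkedComponent is a battle system support component that tracks a stack of marks and displays it through a spawned mark actor.
; On BeginPlay it spawns a BP_A_Mark at the component's world location, with no attachment in this graph, and keeps a reference.
; AddMark adds a quantity clamped between zero and MaxMarks, and ResetMarks clears the count.
; Both then push the count to the actor's UpdateSpheresVisibility.
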(event EventBeginPlay
  (bind _returnvalue (Game|SpawnActorfromClass "/Game/Code/Player/BattleSystem/Support/BP_A_Mark.BP_A_Mark_C" (Math|Transform|MakeTransform (Transformation|GetWorldLocation self) "0, 0, 0" "1,1,1") "Undefined" 0 0))
  (Variables|Default|Setmark _returnvalue))

(event EventTick
  (params (DeltaSeconds :type Float%20%28single-precision%29)))

(fn AddMark
  (params (quantity :type Integer))
  (bind _output_get (Variables|Default|Setmarks (Math|Integer|Clamp(Integer) (+ quantity (Variables|Default|Getmarks)) 0 (LocalVariables|GetmaxMarks))))
  (Default|UpdateSpheresVisibility (Variables|Default|Getmark) _output_get))

(fn ResetMarks
  (bind _output_get (Variables|Default|Setmarks 0))
  (Default|UpdateSpheresVisibility (Variables|Default|Getmark) _output_get))