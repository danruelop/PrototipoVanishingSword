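; Player battle-system support component that marks nearby actors through an expanding push area.
; On BeginPlay it spawns a BP_A_PushArea_01 at the owner, then moves it each tick to the owner's X and Y with sweep.
; GenerateMark grows the area.
; When it reaches level 1, overlapped actors other than the owner that have a BP_C_MarkedComponent receive one mark.
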(event Custom|OnReachLevel1
  (params (overlappedActors :type Array%20of%20Actor%20Object%20References))
  (for _array_element overlappedActors
    (if (not (== _array_element (Components|GetOwner)))
      (Utilities|IsValid (Actor|GetComponentbyClass _array_element "/Game/Code/Player/BattleSystem/Support/BP_C_MarkedComponent.BP_C_MarkedComponent_C")
        (:Is%20Valid
          (Default|AddMark (Actor|GetComponentbyClass _array_element "/Game/Code/Player/BattleSystem/Support/BP_C_MarkedComponent.BP_C_MarkedComponent_C") 1))))))

(event EventBeginPlay
  (bind _returnvalue (Components|GetOwner))
  (bind _returnvalue_2 (Transformation|GetActorTransform _returnvalue))
  (bind _returnvalue_3 (Game|SpawnActorfromClass "/Game/Code/Player/BattleSystem/Support/BP_A_PushArea_01.BP_A_PushArea_01_C" (Math|Transform|MakeTransform (.location _returnvalue_2) (.rotation _returnvalue_2) "1,1,1") "Undefined" 0 0))
  (Variables|Default|SetpushArea _returnvalue_3)
  (EventDispatchers|BindEventtoLevel1onReach (Variables|Default|GetpushArea) (delegate Custom|OnReachLevel1)))

(event EventTick
  (params (DeltaSeconds :type Float%20%28single-precision%29))
  (bind _returnvalue (Components|GetOwner))
  (bind _returnvalue_2 (Transformation|GetActorLocation _returnvalue))
  (Transformation|SetActorLocation (Variables|Default|GetpushArea) (Math|Vector|MakeVector (.x _returnvalue_2) (.y _returnvalue_2) 0.0) true false))

(fn GenerateMark
  (Default|Grow (Variables|Default|GetpushArea)))