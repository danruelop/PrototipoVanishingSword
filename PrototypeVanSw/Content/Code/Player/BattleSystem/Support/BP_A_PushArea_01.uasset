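; A player battle-system push area: a cylinder that grows in width through three levels while ShouldGrow is set.
; Tick drives a LevelState machine, and each level reached recolors the cylinder and broadcasts its overlapping actors through a dispatcher.
; Growth continues after a short pause or resets, while level three always resets and cools down.
; GrowLv3 compares scale against its growth rate instead of a max scale.
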(event Custom|OnLv1Reached
  (params (overlappedActors :type Array%20of%20Actor%20Object%20References))
  ;[1 1 1] Area1 finished
  (Rendering|Material|SetMaterial (Variables|Default|GetCylinder) 0 "/Game/Code/Player/Materials/Mat_Yellow.Mat_Yellow")
  (Variables|Default|SetlevelState "NewEnumerator7")
  (Utilities|FlowControl|Delay 0.2)
  (if (Variables|Default|GetbShouldGrow)
    (Variables|Default|SetlevelState "NewEnumerator2")
    (else
      (CallFunction|RestartArea))))

(event Custom|OnLv2Reached
  (params (OverlappedActors :type Array%20of%20Actor%20Object%20References))
  ;[1 1 1] Area2 finished
  (Rendering|Material|SetMaterial (Variables|Default|GetCylinder) 0 "/Game/Code/Player/Materials/Mat_Orange.Mat_Orange")
  (Variables|Default|SetlevelState "NewEnumerator7")
  (Utilities|FlowControl|Delay 0.2)
  (if (Variables|Default|GetbShouldGrow)
    (Variables|Default|SetlevelState "NewEnumerator3")
    (else
      (CallFunction|RestartArea))))

(event Custom|OnLv3Reached
  (params (NewParam :type Array%20of%20Actor%20Object%20References))
  ;[1 1 1] Area2 finished
  (Rendering|Material|SetMaterial (Variables|Default|GetCylinder) 0 "/Game/Code/Player/Materials/Mat_Red.Mat_Red")
  (Variables|Default|SetlevelState "NewEnumerator7")
  (Utilities|FlowControl|Delay 0.2)
  (CallFunction|RestartArea)
  (Variables|Default|SetlevelState "NewEnumerator7")
  (Utilities|FlowControl|Delay (Variables|Default|GetfCooldownAfterLv3))
  (Variables|Default|SetbShouldGrow false)
  (Variables|Default|SetlevelState "NewEnumerator0"))

(event Custom|Lv1Reached
  (bind _newparam (CallFunction|GetOverlappedActors))
  (Default|CallLevel1onReach _newparam)
  ;[1 1 1] Area1 finished
  (Rendering|Material|SetMaterial (Variables|Default|GetCylinder) 0 "/Game/Code/Player/Materials/Mat_Yellow.Mat_Yellow")
  (Variables|Default|SetlevelState "NewEnumerator7")
  (Utilities|FlowControl|Delay 0.2)
  (if (Variables|Default|GetbShouldGrow)
    (Variables|Default|SetlevelState "NewEnumerator2")
    (else
      (CallFunction|RestartArea))))

(event Custom|Lv2Reached
  (bind _newparam (CallFunction|GetOverlappedActors))
  (Default|CallLevel2onReach _newparam)
  ;[1 1 1] Area2 finished
  (Rendering|Material|SetMaterial (Variables|Default|GetCylinder) 0 "/Game/Code/Player/Materials/Mat_Orange.Mat_Orange")
  (Variables|Default|SetlevelState "NewEnumerator7")
  (Utilities|FlowControl|Delay 0.2)
  (if (Variables|Default|GetbShouldGrow)
    (Variables|Default|SetlevelState "NewEnumerator3")
    (else
      (CallFunction|RestartArea))))

(event Custom|Lv3Reached
  (bind _newparam (CallFunction|GetOverlappedActors))
  (Default|CallLevel3onReach _newparam)
  ;[1 1 1] Area2 finished
  (Rendering|Material|SetMaterial (Variables|Default|GetCylinder) 0 "/Game/Code/Player/Materials/Mat_Red.Mat_Red")
  (Variables|Default|SetlevelState "NewEnumerator7")
  (Utilities|FlowControl|Delay 0.2)
  (CallFunction|RestartArea)
  (Variables|Default|SetlevelState "NewEnumerator7")
  (Utilities|FlowControl|Delay (Variables|Default|GetfCooldownAfterLv3))
  (Variables|Default|SetbShouldGrow false)
  (Variables|Default|SetlevelState "NewEnumerator0"))

(event EventBeginPlay
  (Variables|Default|SetinitialScale (Transformation|GetWorldScale (Variables|Default|GetCylinder))))

(event Collision|EventActorBeginOverlap
  (params (OtherActor :type Actor%20Object%20Reference)))

(event EventTick
  (params (DeltaSeconds :type Float%20%28single-precision%29))
  (CallFunction|Update DeltaSeconds))

(fn ConstructionScript)

(fn Grow
  (params (deltaSeconds :type Float%20%28single-precision%29))
  (switch Utilities|FlowControl|Switch|SwitchonBP_E_AreaLevelState (Variables|Default|GetlevelState)
    (:NewEnumerator0
      (CallFunction|GrowLv1 deltaSeconds :!label _label))
    (:NewEnumerator1
      (goto _label))
    (:NewEnumerator2
      (CallFunction|GrowLv2 deltaSeconds))
    (:NewEnumerator3
      (CallFunction|GrowLv3 deltaSeconds))))

(fn Update
  (params (deltaSeconds :type Float%20%28single-precision%29))
  (if (Variables|Default|GetbShouldGrow)
    (CallFunction|Grow deltaSeconds)))

(fn RestartArea
  (Transformation|SetWorldScale3D (Variables|Default|GetCylinder) (Variables|Default|GetinitialScale))
  (Rendering|Material|SetMaterial (Variables|Default|GetCylinder) 0 "/Game/Code/Player/Materials/Female_Mat.Female_Mat")
  (Utilities|FlowControl|Sequence))

(fn GetOverlappedActors
  (return (Collision|GetOverlappingActors (Variables|Default|GetCylinder) "/Script/Engine.Actor" :!class /Script/Engine.PrimitiveComponent)))

(fn SetShouldGrow
  (params (NewParam :type Boolean))
  (Variables|Default|SetbShouldGrow NewParam))

(fn GrowLv1
  (params (DeltaSeconds :type Float%20%28single-precision%29))
  (bind _flv1increasepersecond (Variables|Default|GetfLv1IncreasePerSecond))
  (bind _cylinder (Variables|Default|GetCylinder))
  (bind _returnvalue (Transformation|GetWorldScale _cylinder))
  (bind _returnvalue_2 (* _flv1increasepersecond DeltaSeconds))
  (bind _returnvalue_3 (+ _returnvalue_2 (.x _returnvalue)))
  (if (>= (.x (Transformation|GetWorldScale (Variables|Default|GetCylinder))) (Variables|Default|GetfLv1MaxScale))
    ;[1 1 1] Reached lv 1
    (CallFunction|Lv1Reached)
    (else
      (Transformation|SetWorldScale3D (Variables|Default|GetCylinder) (Math|Vector|MakeVector _returnvalue_3 _returnvalue_3 (.z _returnvalue))))))

(fn GrowLv2
  (params (DeltaSeconds :type Float%20%28single-precision%29))
  (bind _cylinder (Variables|Default|GetCylinder))
  (bind _flv2increasepersecond (Variables|Default|GetfLv2IncreasePerSecond))
  (bind _returnvalue (Transformation|GetWorldScale _cylinder))
  (bind _returnvalue_2 (* _flv2increasepersecond DeltaSeconds))
  (bind _returnvalue_3 (+ _returnvalue_2 (.x _returnvalue)))
  (if (>= (.x (Transformation|GetWorldScale (Variables|Default|GetCylinder))) (Variables|Default|GetfLv2MaxScale))
    ;[1 1 1] Reached lv 2
    (CallFunction|Lv2Reached)
    (else
      (Transformation|SetWorldScale3D (Variables|Default|GetCylinder) (Math|Vector|MakeVector _returnvalue_3 _returnvalue_3 (.z _returnvalue))))))

(fn GrowLv3
  (params (DeltaSeconds :type Float%20%28single-precision%29))
  (bind _cylinder (Variables|Default|GetCylinder))
  (bind _flv3increasepersecond (Variables|Default|GetfLv3IncreasePerSecond))
  (bind _returnvalue (Transformation|GetWorldScale _cylinder))
  (bind _returnvalue_2 (* _flv3increasepersecond DeltaSeconds))
  (bind _returnvalue_3 (+ _returnvalue_2 (.x _returnvalue)))
  (if (>= (.x (Transformation|GetWorldScale (Variables|Default|GetCylinder))) (Variables|Default|GetfLv3IncreasePerSecond))
    ;[1 1 1] Reached lv 3
    (CallFunction|Lv3Reached)
    (else
      (Transformation|SetWorldScale3D (Variables|Default|GetCylinder) (Math|Vector|MakeVector _returnvalue_3 _returnvalue_3 (.z _returnvalue))))))