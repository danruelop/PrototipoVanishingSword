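; Actor that displays a floating mark counter of up to three spheres on its owning actor in the battle system.
; Init adds one mark, VariateMarksQuantity adjusts the count, and ResetMarks clears it, with each updating which spheres are visible.
; Every Tick it moves itself to the mark point supplied by the owner through the BP_I_Marked interface.
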(event EventBeginPlay
  (CallFunction|VariateMarksQuantity))

(event Collision|EventActorBeginOverlap
  (params (OtherActor :type Actor%20Object%20Reference)))

(event EventTick
  (params (DeltaSeconds :type Float%20%28single-precision%29))
  (CallFunction|UpdateSpheresPosition))

(fn ConstructionScript)

(fn ResetMarks
  (params (NewParam :type Integer))
  (Variables|Default|SetnumberOfSpheres 0)
  (CallFunction|UpdateSpheresVisibility))

(fn VariateMarksQuantity
  (params (NewParam :type Integer))
  (bind _output_get (Variables|Default|SetnumberOfSpheres (+ NewParam (Variables|Default|GetnumberOfSpheres))))
  (CallFunction|UpdateSpheresVisibility _output_get))

(fn UpdateSpheresVisibility
  (params (NewParam :type Integer))
  (switch int NewParam
    (:Default
      (Rendering|SetVisibility (Variables|Default|GetSphere1) false false :!label _label)
      (Rendering|SetVisibility (Variables|Default|GetSphere2) false false)
      (Rendering|SetVisibility (Variables|Default|GetSphere3) false false))
    (:0
      (goto _label))
    (:1
      (Rendering|SetVisibility (Variables|Default|GetSphere1) true false)
      (Rendering|SetVisibility (Variables|Default|GetSphere2) false false)
      (Rendering|SetVisibility (Variables|Default|GetSphere3) false false))
    (:2
      (Rendering|SetVisibility (Variables|Default|GetSphere1) true false)
      (Rendering|SetVisibility (Variables|Default|GetSphere2) true false)
      (Rendering|SetVisibility (Variables|Default|GetSphere3) false false))
    (:3
      (Rendering|SetVisibility (Variables|Default|GetSphere1) true false)
      (Rendering|SetVisibility (Variables|Default|GetSphere2) true false)
      (Rendering|SetVisibility (Variables|Default|GetSphere3) true false))))

(fn UpdateSpheresPosition
  (bind _returnvalue (Components|GetOwner))
  (Utilities|IsValid _returnvalue
    (:Is%20Valid
      (if (Utilities|DoesObjectImplementInterface _returnvalue "/Game/Code/Player/BattleSystem/Support/BP_I_Marked.BP_I_Marked_C")
        (Utilities|FlowControl|Sequence
          (:then_0
            (bind _marklocation (Class|BPIMarked|GetMarkPoint(Message) _returnvalue))
            (LocalVariables|SetmarkLocation _marklocation))
          (:then_1
            (Transformation|SetActorLocation self (LocalVariables|GetmarkLocation) false false)))))))

(fn Init
  (params (ownerActorHeight :type Float%20%28single-precision%29))
  (Variables|Default|SetownerActorHeight ownerActorHeight)
  (CallFunction|VariateMarksQuantity 1))