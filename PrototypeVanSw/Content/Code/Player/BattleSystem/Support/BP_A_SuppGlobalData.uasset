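; BP_A_SuppGlobalData is an actor in the player battle system's support code that holds a shared list of marked actors.
; AddMarkedActor accepts only actors that carry a BP_C_MarkedComponent and skips any already in the list.
; Companion functions remove an actor, test membership and return the list, while the event graph and construction script contain no logic.
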(event EventBeginPlay)

(event Collision|EventActorBeginOverlap
  (params (OtherActor :type Actor%20Object%20Reference)))

(event EventTick
  (params (DeltaSeconds :type Float%20%28single-precision%29)))

(fn ConstructionScript)

(fn AddMarkedActor
  (params (actor :type Actor%20Object%20Reference))
  (Utilities|IsValid (Actor|GetComponentbyClass actor "/Game/Code/Player/BattleSystem/Support/BP_C_MarkedComponent.BP_C_MarkedComponent_C")
    (:Is%20Valid
      (if (not (Utilities|Array|ContainsItem (Variables|Default|GetmarkedActors) actor))
        (Utilities|Array|Add (Variables|Default|GetmarkedActors) actor)))))

(fn RemoveMarkedActor
  (params (actor :type Actor%20Object%20Reference))
  (Utilities|Array|RemoveItem (Variables|Default|GetmarkedActors) actor))

(fn ContainsMarkedActor
  (params (actor :type Actor%20Object%20Reference))
  (return (Utilities|Array|ContainsItem (Variables|Default|GetmarkedActors) actor)))

(fn GetMarkedActors
  (return (Variables|Default|GetmarkedActors)))