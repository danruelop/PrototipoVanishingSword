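; BP_A_Dummy_01 is a target dummy actor for the player battle system that displays damage taken and reacts to pushes.
; ApplyDamage shows the latest damage value on a TextRender and restarts a cooldown, which Tick counts down to reset the text to zero.
; Push applies a scaled directional impulse to the Body, and GetMarkPoint returns the StatusPos world location.
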(event EventBeginPlay)

(event Collision|EventActorBeginOverlap
  (params (OtherActor :type Actor%20Object%20Reference)))

(event EventTick
  (params (DeltaSeconds :type Float%20%28single-precision%29))
  (bind _output_get (Variables|Default|SetfCurrentCooldown (+ (* DeltaSeconds -1.0) (Variables|Default|GetfCurrentCooldown))))
  (if (<= _output_get 0.0)
    (CallFunction|Restart)
    (Rendering|Components|TextRender|SetText (Variables|Default|GetTextRender) (Utilities|Text|ToText(Integer) 0))))

(event EventApplyDamage
  (params (DPSBasicAttackDamage :type Integer) (attacker :type Actor%20Object%20Reference))
  (Rendering|Components|TextRender|SetText (Variables|Default|GetTextRender) (Utilities|Text|ToText(Integer) DPSBasicAttackDamage))
  (CallFunction|ResetCooldown))

(event EventPush
  (params (fForceMultiplier :type Float%20%28single-precision%29) (direction :type Vector :default "0, 0, 0"))
  (Physics|AddImpulse (Variables|Default|GetBody) (* direction (* fForceMultiplier 99988.0)) "None" false))

(fn ConstructionScript)

(fn ResetCooldown
  (Variables|Default|SetfCurrentCooldown (Variables|Default|GetfCooldown)))

(fn Restart
  (CallFunction|ResetCooldown))

(fn GetMarkPoint
  (return (Transformation|GetWorldLocation (Variables|Default|GetstatusPos))))