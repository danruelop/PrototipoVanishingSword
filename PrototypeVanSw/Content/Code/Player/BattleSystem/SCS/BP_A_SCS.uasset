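; SCS actor that tracks the players' shared consecutive-hit meter and loop level, plus the DPS player's charged attack.
; Confirmed hits fill the meter, rolling surplus into new loops, while attacks without hits restart it to the minimum loop.
; An idle countdown, paused while charging, drains the meter and fires events.
; Tick also advances three charge levels, refreshes debug text and keeps the actor midway between both players.
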(event EventBeginPlay
  (Variables|Countdown|SetcurrentCountdown (Variables|Countdown|GetcountdownUntilReset))
  (if (<= (Variables|Countdown|GetconsecutiveAccumulatedDecrementBySecond) 0.0)
    (Variables|Countdown|SetconsecutiveAccumulatedDecrementBySecond 0.5)))

(event Collision|EventActorBeginOverlap
  (params (OtherActor :type Actor%20Object%20Reference)))

(event EventTick
  (params (DeltaSeconds :type Float%20%28single-precision%29))
  (Countdown|UpdateCountdown DeltaSeconds)
  ;[1 1 1] CHARGING
  (ChargedAttack|UpdateChargingAttack DeltaSeconds)
  ;[1 1 1] Debug
  (Debug|UpdateText)
  (Debug|UpdatePosition))

(fn ConstructionScript)

(fn Confirm
  (params (confirmedValue :type Float%20%28single-precision%29))
  (if (Variables|Default|GetconfirmationInCurrentActivatedAttackAreaCourse)
    (if (not (Variables|Default|GetbIsLimitedToOneConsecutivePerAttack))
      (Variables|Default|SetconfirmationInCurrentActivatedAttackAreaCourse true :!label _label)
      (CallFunction|AugmentConsecutive confirmedValue)
      (Default|CallOnConfirmation))
    (else
      (goto _label))))

(fn Miss
  (CallFunction|Restart))

(fn Restart
  (Utilities|FlowControl|Sequence
    (:then_0
      (Variables|Default|SetconsecutiveAccumulated 0.0)
      (Variables|Default|SetcurrentLoop (Variables|Bonus|GetminimumLoopLevelBonus)))
    (:then_1
      (Countdown|ResetCountdown))
    (:then_2
      (Default|CallOnRestarted))))

(fn OnAttackHitboxActivated
  (Variables|Default|SetconfirmationInCurrentActivatedAttackAreaCourse false))

(fn OnAttackHitboxDeactivated
  (Countdown|ResetCountdown)
  (if (not (Variables|Default|GetconfirmationInCurrentActivatedAttackAreaCourse))
    (CallFunction|Miss)))

(fn AugmentConsecutive
  (params (_by :type Float%20%28single-precision%29))
  (LocalVariables|Setby _by)
  (bind _output_get (LocalVariables|SetconsecutiveAccumulatedSurplus (- (+ (Variables|Default|GetconsecutiveAccumulated) (LocalVariables|Getby)) (Variables|Default|GetconsecutiveNeededToLoop))))
  (if (>= _output_get 0.0)
    ;[1 1 1] Make a loop
    (Utilities|FlowControl|Sequence
      (:then_0
        (Variables|Default|SetconsecutiveAccumulated (LocalVariables|GetconsecutiveAccumulatedSurplus)))
      (:then_1
        (Variables|Default|SetcurrentLoop (+ (Variables|Default|GetcurrentLoop) 1)))
      (:then_2
        (Default|CallOnLoopPlus (Variables|Default|GetcurrentLoop))))
    (else
      (Variables|Default|SetconsecutiveAccumulated (+ (Variables|Default|GetconsecutiveAccumulated) (LocalVariables|Getby))))))

(fn OnAttackAreaOverlap
  (params (actorHit :type Actor%20Object%20Reference%20%28by%20ref%29) (confirmedValue :type Float%20%28single-precision%29))
  (Utilities|Casting|CastToBP_Player actorHit
    (:CastFailed
      (if (Utilities|DoesObjectImplementInterface actorHit "/Game/Code/BPI_OnHit.BPI_OnHit_C")
        (CallFunction|Confirm confirmedValue)))))

(fn AddBonusConsecutive
  (params (quantity :type Float%20%28single-precision%29))
  (bind _output_get (Variables|Bonus|SetconsecutiveBonus (+ quantity (Variables|Bonus|GetconsecutiveBonus))))
  (bind _newparam1 (Bonus|ClampBonus _output_get))
  (Variables|Bonus|SetconsecutiveBonus _newparam1))

(fn AddBonusLoop
  (params (quantity :type Integer))
  (bind _output_get (Variables|Bonus|SetminimumLoopLevelBonus (+ quantity (Variables|Bonus|GetminimumLoopLevelBonus))))
  (if (< _output_get 0)
    (Variables|Bonus|SetminimumLoopLevelBonus 0)))

(fn ClampBonus
  (params (NewParam :type Float%20%28single-precision%29))
  (if (< NewParam 0.0)
    (return 0.0)
    (else
      (return NewParam))))

(fn UpdateCountdown
  (params (deltaSeconds :type Float%20%28single-precision%29))
  (Utilities|FlowControl|Sequence
    (:then_0
      (bind _newparam (CallFunction|IsSomeAccumulated))
      (if _newparam
        (if (not (Variables|ChargedAttack|GetbIsChargingAttack))
          (if true
            (bind _output_get (Variables|Countdown|SetcurrentCountdown (- (Variables|Countdown|GetcurrentCountdown) deltaSeconds)))
            (if (< _output_get 0.0)
              (Countdown|ReduceConsecutiveAccumulatedbyCountdown (* deltaSeconds (Variables|Countdown|GetconsecutiveAccumulatedDecrementBySecond)))
              (LocalVariables|SetconsecutiveAccumulatedByCountdownReduced true))))))
    (:then_1
      (if (LocalVariables|GetconsecutiveAccumulatedByCountdownReduced)
        (if (not (Variables|Default|GetbAlreadyCalledEvent_OnCountDownStartDecreasing))
          (Variables|Default|SetbAlreadyCalledEvent_OnCountDownStartDecreasing true)
          (Default|CallOnCountdownStartsDecreasing))
        (elif (Variables|Default|GetbAlreadyCalledEvent_OnCountDownStartDecreasing)
          (Variables|Default|SetbAlreadyCalledEvent_OnCountDownStartDecreasing false)
          (Default|CallOnCountdownEndsDecreasing))))))

(fn ReduceConsecutiveAccumulatedbyCountdown
  (params (By :type Float%20%28single-precision%29))
  (bind _output_get (Variables|Default|SetconsecutiveAccumulated (- (Variables|Default|GetconsecutiveAccumulated) By)))
  (if (<= _output_get 0.0)
    (CallFunction|Restart)))

(fn ResetCountdown
  (Variables|Countdown|SetcurrentCountdown (Variables|Countdown|GetcountdownUntilReset)))

(fn UpdateText
  (Rendering|Components|TextRender|SetText (Variables|Default|GetLoopText) (Utilities|Text|ToText(Integer) (Variables|Default|GetcurrentLoop)))
  (Rendering|Components|TextRender|SetText (Variables|Default|GetConsecutiveText) (Utilities|Text|ToText(Float) (Variables|Default|GetconsecutiveAccumulated) "HalfToEven")))

(fn IsSomeAccumulated
  (return (or (> (Variables|Default|GetcurrentLoop) 0) (> (Variables|Default|GetconsecutiveAccumulated) 0.0))))

(fn StartCharging
  (Variables|ChargedAttack|SetbIsChargingAttack true))

(fn EndCharging
  (Variables|ChargedAttack|SetbShouldStopAtNextChargedLv false)
  (Variables|ChargedAttack|SetbIsChargingAttack false)
  (Variables|ChargedAttack|SetfChargedAttackAccumulated 0.0)
  (Utilities|FlowControl|Sequence
    (:then_0
      (bind _returnvalue (Actor|GetActorOfClass "/Game/Code/Player/BP_FemalePlayer.BP_FemalePlayer_C"))
      (Default|TryDoingChargingAttack _returnvalue))
    (:then_1
      (bind _returnvalue_2 (Actor|GetActorOfClass "/Game/Code/Player/BP_MalePlayer.BP_MalePlayer_C"))
      (Default|TryDoingChargingAttack _returnvalue_2))))

(fn UpdatePosition
  (bind _returnvalue (Actor|GetActorOfClass "/Game/Code/Player/BP_MalePlayer.BP_MalePlayer_C"))
  (bind _returnvalue_2 (Actor|GetActorOfClass "/Game/Code/Player/BP_FemalePlayer.BP_FemalePlayer_C"))
  (Transformation|SetActorLocation self (/ (+ (Transformation|GetActorLocation _returnvalue_2) (Transformation|GetActorLocation _returnvalue)) 2) true false))

(fn ShowFrozenUISCS
  (params (frozen :type Boolean)))

(fn UpdateChargingAttack
  (params (DeltaSeconds :type Float%20%28single-precision%29))
  ;[1 1 1] update each player
  (bind _player (CallFunction|GetSuppPlayer))
  (Variables|/Script/PrototypeVanSw.PrototypeVanSwCharacter|SetmBIsCharginAttack _player false)
  (if (Variables|ChargedAttack|GetbIsChargingAttack)
    (bind _player_2 (CallFunction|GetDPSPlayer))
    (Variables|/Script/PrototypeVanSw.PrototypeVanSwCharacter|SetmBIsCharginAttack _player_2 true)
    (Variables|ChargedAttack|SetfChargedAttackAccumulated (+ DeltaSeconds (Variables|ChargedAttack|GetfChargedAttackAccumulated)))
    (bind _player_3 (CallFunction|GetDPSPlayer))
    (LocalVariables|SetdpsPlayer _player_3)
    (if (>= (Variables|ChargedAttack|GetfChargedAttackAccumulated) (Variables|ChargedAttack|GetfChargedAttackCountdownLv3))
      (Default|ActivateChargingAttackLv3 (LocalVariables|GetdpsPlayer))
      (bind _output_get (Variables|ChargedAttack|SetchargingState "NewEnumerator5"))
      (ChargedAttack|OnChargingLevelReached _output_get)
      (elif (>= (Variables|ChargedAttack|GetfChargedAttackAccumulated) (Variables|ChargedAttack|GetfChargedAttackCountdownLv2))
        (Default|ActivateChargingAttackLv2 (LocalVariables|GetdpsPlayer))
        (bind _output_get_2 (Variables|ChargedAttack|SetchargingState "NewEnumerator3"))
        (ChargedAttack|OnChargingLevelReached _output_get_2)
        (elif (>= (Variables|ChargedAttack|GetfChargedAttackAccumulated) (Variables|ChargedAttack|GetfChargedAttackCountdownLv1))
          (Default|ActivateChargingAttackLv1 (LocalVariables|GetdpsPlayer))
          (bind _output_get_3 (Variables|ChargedAttack|SetchargingState "NewEnumerator2"))
          (ChargedAttack|OnChargingLevelReached _output_get_3)
          (else
            (Variables|ChargedAttack|SetchargingState "NewEnumerator4")))))
    (else
      (Variables|ChargedAttack|SetchargingState "NewEnumerator0")
      (bind _player_4 (CallFunction|GetDPSPlayer))
      (Variables|/Script/PrototypeVanSw.PrototypeVanSwCharacter|SetmBIsCharginAttack _player_4 false))))

(fn GetDPSPlayer
  (bind _outactors (Actor|GetAllActorsOfClass "/Game/Code/Player/BP_Player.BP_Player_C"))
  (for _array_element _outactors
    (if (Variables|/Game/Code/Player/BP_Player.BP_Player_C|GetbIsDPS _array_element)
      (return _array_element))))

(fn GetSuppPlayer
  (bind _outactors (Actor|GetAllActorsOfClass "/Game/Code/Player/BP_Player.BP_Player_C"))
  (for _array_element _outactors
    (if (not (Variables|/Game/Code/Player/BP_Player.BP_Player_C|GetbIsDPS _array_element))
      (return _array_element))))

(fn OnChargingLevelReached
  (params (state :type BP_E_ChargingStates%20Enum :default "NewEnumerator0"))
  (Variables|ChargedAttack|SetchargingState state)
  (if (Variables|ChargedAttack|GetbShouldStopAtNextChargedLv)
    (ChargedAttack|EndCharging)))