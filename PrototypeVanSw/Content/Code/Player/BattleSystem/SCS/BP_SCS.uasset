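; BP_SCS is a player battle-system Blueprint that tracks consecutive successful attacks, with a loop level shown beside the count.
; Attack hitbox activation opens a window where the first overlap with a non-player BPI_OnHit actor adds one plus a bonus, wrapping at a threshold.
; A hitbox closing unconfirmed resets the count, countdown and loop, the latter to its bonus minimum.
; Bonuses clamp at zero, Tick refreshes both texts, and nothing here increments the loop.
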(event EventBeginPlay)

(event Collision|EventActorBeginOverlap
  (params (OtherActor :type Actor%20Object%20Reference)))

(event EventTick
  (params (DeltaSeconds :type Float%20%28single-precision%29))
  (CallFunction|UpdateText))

(fn ConstructionScript)

(fn Confirm
  (Utilities|FlowControl|Sequence
    (:then_1
      (if (not (Variables|Default|GetconfirmationInCurrentActivateCourse))
        (Variables|Default|SetconfirmationInCurrentActivateCourse true)
        (CallFunction|AugmentConsecutive (+ (Variables|Bonus|GetconsecutiveBonus) 1))))))

(fn Miss
  (CallFunction|Restart))

(fn Restart
  (Utilities|FlowControl|Sequence
    (:then_0
      (Variables|Default|SetcurrentconsecutiveCount 0)
      (Variables|Default|SetcurrentLoop (Variables|Bonus|GetminimumLoopLevelBonus))
      (Development|PrintString "Restart SCS"))
    (:then_1
      (Countdown|ResetCountdown))))

(fn OnAttackHitboxActivated
  (Variables|Default|SetconfirmationInCurrentActivateCourse false))

(fn OnAttackHitboxDeactivated
  (if (not (Variables|Default|GetconfirmationInCurrentActivateCourse))
    (CallFunction|Miss)))

(fn AugmentConsecutive
  (params (_by :type Integer))
  (LocalVariables|Setby _by)
  (Utilities|FlowControl|Sequence
    (:then_0
      (bind _output_get (Variables|Default|SetcurrentconsecutiveCount (+ (Variables|Default|GetcurrentconsecutiveCount) (LocalVariables|Getby))))
      (if (>= _output_get (Variables|Default|GetconsecutiveNeededToLoop))
        (Variables|Default|SetcurrentconsecutiveCount (- (LocalVariables|Getby) 1))))))

(fn OnAttackAreaOverlap
  (params (actorHit :type Actor%20Object%20Reference%20%28by%20ref%29))
  (Utilities|Casting|CastToBP_Player actorHit
    (:CastFailed
      (if (Utilities|DoesObjectImplementInterface actorHit "/Game/Code/BPI_OnHit.BPI_OnHit_C")
        (CallFunction|Confirm)))))

(fn AddBonusConsecutive
  (params (quantity :type Integer))
  (bind _output_get (Variables|Bonus|SetconsecutiveBonus (+ quantity (Variables|Bonus|GetconsecutiveBonus))))
  (bind _newparam1 (Bonus|ClampBonus _output_get))
  (Variables|Bonus|SetconsecutiveBonus _newparam1))

(fn AddBonusLoop
  (params (quantity :type Integer))
  (bind _output_get (Variables|Bonus|SetminimumLoopLevelBonus (+ quantity (Variables|Bonus|GetminimumLoopLevelBonus))))
  (bind _newparam1 (Bonus|ClampBonus _output_get))
  (Variables|Bonus|SetminimumLoopLevelBonus _newparam1))

(fn ClampBonus
  (params (NewParam :type Integer))
  (if (< NewParam 0)
    (return 0)
    (else
      (return NewParam))))

(fn ResetCountdown
  (Variables|Countdown|SetcurrentCountdown 0))

(fn UpdateText
  (Rendering|Components|TextRender|SetText (Variables|Default|GetLoopText) (Utilities|Text|ToText(Integer) (Variables|Default|GetcurrentLoop)))
  (Rendering|Components|TextRender|SetText (Variables|Default|GetConsecutiveText) (Utilities|Text|ToText(Integer) (Variables|Default|GetcurrentconsecutiveCount))))