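; BP_A_VisualClueSCSLoop is a short-lived looping visual clue actor for the battle system (SCS) that follows the actor it is attached to.
; Each tick it snaps to that actor's location, spins around yaw by a per-frame step, and raises five spheres at a set upward velocity.
; On BeginPlay it increments the player's active loop-clue counter, then decrements it and destroys itself after LifeTime.
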(event EventBeginPlay
  (Utilities|FlowControl|Sequence
    (:then_0
      (CallFunction|PopulateAllSpheres))
    (:then_1
      (bind _asbp_player (Utilities|Casting|CastToBP_Player (Variables|Default|GetactorAttachedTo)))
      (Variables|/Game/Code/Player/BP_Player.BP_Player_C|SetcurrentSpawnedLoopVisualClues _asbp_player (+ (Variables|/Game/Code/Player/BP_Player.BP_Player_C|GetcurrentSpawnedLoopVisualClues _asbp_player) 1)))
    (:then_2
      (Utilities|FlowControl|Delay (Variables|Default|GetlifeTime))
      (bind _asbp_player_2 (Utilities|Casting|CastToBP_Player (Variables|Default|GetactorAttachedTo))
        (:then
          (Variables|/Game/Code/Player/BP_Player.BP_Player_C|SetcurrentSpawnedLoopVisualClues _asbp_player_2 (+ (Variables|/Game/Code/Player/BP_Player.BP_Player_C|GetcurrentSpawnedLoopVisualClues _asbp_player_2) -1)))
        (:CastFailed
          _))
      (Actor|DestroyActor))))

(event Collision|EventActorBeginOverlap
  (params (OtherActor :type Actor%20Object%20Reference)))

(event EventTick
  (params (DeltaSeconds :type Float%20%28single-precision%29))
  (CallFunction|Move DeltaSeconds))

(fn ConstructionScript)

(fn Move
  (params (deltaSeconds :type Float%20%28single-precision%29))
  (Utilities|FlowControl|Sequence
    (:then_0
      (for _array_element (Variables|Default|GetallSpheres)
        (Transformation|SetWorldLocation _array_element (Math|Vector|MakeVector (.x (Transformation|GetWorldLocation _array_element)) (.y (Transformation|GetWorldLocation _array_element)) (+ (.z (Transformation|GetWorldLocation _array_element)) (* deltaSeconds (Variables|Default|GetupVelocityPerSecond)))) false false)))
    (:then_1
      (Transformation|SetActorLocation self (Transformation|GetActorLocation (Variables|Default|GetactorAttachedTo)) false false))
    (:then_2
      (Transformation|SetActorRotation self (Math|Rotator|MakeRotator 0.0 0.0 (+ (.yaw (Transformation|GetActorRotation self)) (Variables|Default|GetrotationPerSecond)))))))

(fn PopulateAllSpheres
  (Utilities|FlowControl|Sequence
    (:then_0
      (Utilities|Array|Add (Variables|Default|GetallSpheres) (Variables|Default|GetSphere)))
    (:then_1
      (Utilities|Array|Add (Variables|Default|GetallSpheres) (Variables|Default|GetSphere1)))
    (:then_2
      (Utilities|Array|Add (Variables|Default|GetallSpheres) (Variables|Default|GetSphere2)))
    (:then_3
      (Utilities|Array|Add (Variables|Default|GetallSpheres) (Variables|Default|GetSphere3)))
    (:then_4
      (Utilities|Array|Add (Variables|Default|GetallSpheres) (Variables|Default|GetSphere4)))))