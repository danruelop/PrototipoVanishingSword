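; Actor component in the player battle system that holds base and bonus damage values and reports the resulting total.
; GetDamage returns base plus bonus, falling back to a minimum total when the sum is zero or below; BeginPlay defaults that minimum to one if non-positive.
; ClampDamageBonus adds any non-positive total onto the bonus, which lowers a negative sum further instead of clamping it.
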(event EventBeginPlay
  (if (<= (Variables|Default|GetfMinimumTotalDamage) 0.0)
    (Variables|Default|SetfMinimumTotalDamage 1.0)))

(event EventTick
  (params (DeltaSeconds :type Float%20%28single-precision%29)))

(fn GetDamage
  (bind _fdamagebase (Variables|Default|GetfDamageBase))
  (bind _fdamagebonus (Variables|Default|GetfDamageBonus))
  (bind _returnvalue (+ _fdamagebase _fdamagebonus))
  (if (<= _returnvalue 0.0)
    (return (Variables|Default|GetfMinimumTotalDamage))
    (else
      (return _returnvalue))))

(fn ClampDamageBonus
  (if (<= (+ (Variables|Default|GetfDamageBonus) (Variables|Default|GetfDamageBase)) 0.0)
    (Variables|Default|SetfDamageBonus (+ (Variables|Default|GetfDamageBonus) (+ (Variables|Default|GetfDamageBonus) (Variables|Default|GetfDamageBase))))))