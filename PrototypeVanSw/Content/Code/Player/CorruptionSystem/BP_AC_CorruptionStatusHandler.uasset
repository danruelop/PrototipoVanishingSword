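; Actor component for the player's corruption system that tracks which of three bar segments the current corruption status is in.
; Init stores the status and bar width point; Update refreshes the point and derives a segment index from SegmentWidth.
; An index change only prints to screen, as ChangeStatus and ActivateStatus are empty stubs.
; ClampStatusQuantity is unused and effectively clamps only at zero, since its upper check compares the input to itself.
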(event EventBeginPlay)

(event EventTick
  (params (DeltaSeconds :type Float%20%28single-precision%29)))

(fn ChangeStatus)

(fn ClampStatusQuantity
  (params (statusQuantity :type Integer))
  (LocalVariables|SetstatusQuantityOut statusQuantity)
  (Utilities|FlowControl|Sequence
    (:then_0
      (if (> (LocalVariables|GetstatusQuantityOut) (Variables|Default|GetstatusQuantity))
        (LocalVariables|SetstatusQuantityOut (Variables|Default|GetstatusQuantity))))
    (:then_1
      (if (< (LocalVariables|GetstatusQuantityOut) 0)
        (LocalVariables|SetstatusQuantityOut 0)))
    (:then_2
      (return (LocalVariables|GetstatusQuantityOut)))))

(fn ActivateStatus)

(fn Init
  (params (status :type Array%20of%20BP_E_CorruptionStatusTypes%20Enums :default "NewEnumerator0") (currentBarWidthPoint :type Float%20%28single-precision%29))
  (Variables|Default|Setstatus status)
  (Variables|Default|SetcurrentBarWidthPoint currentBarWidthPoint))

(fn Update
  (params (currentBarWidthPoint :type Float%20%28single-precision%29))
  (Variables|Default|SetcurrentBarWidthPoint currentBarWidthPoint)
  (CallFunction|UpdateStatusIndex))

(fn UpdateStatusIndex
  (Utilities|FlowControl|Sequence
    (:then_0
      (if (< (Variables|Default|GetcurrentBarWidthPoint) (Variables|Default|GetsegmentWidth))
        (LocalVariables|Setindex 0)
        (elif (< (Variables|Default|GetcurrentBarWidthPoint) (* 2 (Variables|Default|GetsegmentWidth)))
          (LocalVariables|Setindex 1)
          (else
            (LocalVariables|Setindex 2)))))
    (:then_1
      (if (!= (LocalVariables|Getindex) (Variables|Default|GetcurrentIndex))
        (Development|PrintString (Utilities|String|ToString(Integer) (LocalVariables|Getindex))))
      (Variables|Default|SetcurrentIndex (LocalVariables|Getindex)))))