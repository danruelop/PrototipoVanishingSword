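; Actor component that gives its owner a chance to drop a corruption or health pickup when destroyed.
; On EndPlay with reason Destroyed, it rolls against a base chance plus the pickup bonus rate of the last attacker, if that is a player.
; A successful roll spawns one of four equally weighted classes, normal or big, at the owner's location.
; UpdateLastAttacker stores the attacker used for that bonus.
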(event EventBeginPlay)

(event EventTick
  (params (DeltaSeconds :type Float%20%28single-precision%29)))

(event EventEndPlay
  (params (EndPlayReason :type EEndPlayReason%20Enum :default "Destroyed"))
  (switch Utilities|FlowControl|Switch|SwitchonEEndPlayReason EndPlayReason
    (:Destroyed
      (CallFunction|TrySpawnPickup))))

(fn TrySpawnPickup
  (Utilities|FlowControl|Sequence
    (:then_0
      (Utilities|IsValid (Variables|Default|GetlastAttacker)
        (:Is%20Valid
          (bind _asbp_player (Utilities|Casting|CastToBP_Player (Variables|Default|GetlastAttacker)))
          (LocalVariables|SetfRatebonus (Variables|/Game/Code/Player/BP_Player.BP_Player_C|GetfPickupBonusRate _asbp_player)))))
    (:then_1
      (if (<= (Math|Random|RandomFloatinRange 0.0 1.0) (+ (Variables|Default|GetfChanceRate) (LocalVariables|GetfRatebonus)))
        (bind _newparam (CallFunction|GetPickupClasstoSpawn))
        (Game|SpawnActorfromClass _newparam (Math|Transform|MakeTransform (.location (Transformation|GetWorldTransform (Variables|/Script/Engine.Actor|GetRootComponent (Components|GetOwner)))) "0, 0, 0" "1,1,1") "Undefined" 0 0)))))

(fn GetPickupClasstoSpawn
  (LocalVariables|SetfRandom (Math|Random|RandomFloatinRange 0.0 4.0))
  (Utilities|FlowControl|Sequence
    (:then_0
      (if (<= (LocalVariables|GetfRandom) 1.0)
        (LocalVariables|Setclass "/Game/Code/Player/CorruptionSystem/BP_PickUpCorruption.BP_PickUpCorruption_C")))
    (:then_1
      (if (and (<= (LocalVariables|GetfRandom) 2.0) (> (LocalVariables|GetfRandom) 1.0))
        (LocalVariables|Setclass "/Game/Code/Player/CorruptionSystem/BP_PickUpCorruptionBig.BP_PickUpCorruptionBig_C")))
    (:then_2
      (if (and (<= (LocalVariables|GetfRandom) 3.0) (> (LocalVariables|GetfRandom) 2.0))
        (LocalVariables|Setclass "/Game/Code/Player/CorruptionSystem/BP_PickUpHealth.BP_PickUpHealth_C")))
    (:then_3
      (if (and (<= (LocalVariables|GetfRandom) 4.0) (> (LocalVariables|GetfRandom) 3.0))
        (LocalVariables|Setclass "/Game/Code/Player/CorruptionSystem/BP_PickUpHealthBig.BP_PickUpHealthBig_C")))
    (:then_4
      (return (LocalVariables|Getclass)))))

(fn UpdateLastAttacker
  (params (attacker :type Actor%20Object%20Reference))
  (Utilities|IsValid attacker
    (:Is%20Valid
      (Variables|Default|SetlastAttacker attacker))))