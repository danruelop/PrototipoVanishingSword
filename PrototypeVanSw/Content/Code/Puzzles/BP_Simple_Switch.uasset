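; BP_Simple_Switch is a one-shot puzzle switch that the player activates with the DPS attack zone.
; When BP_Player overlaps the Box and its DPSAttackZone touches that component, a DoOnce sets IsActive, calls ActivateSwitch and swaps the cone to its "on" material.
; Independently, a timeline started on BeginPlay lerps the cone's relative location from its initial position toward EndPosition.
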(event OnComponentBeginOverlap(Box)
  (params (OverlappedComponent :type Primitive%20Component%20Object%20Reference) (OtherActor :type Actor%20Object%20Reference) (OtherComp :type Primitive%20Component%20Object%20Reference) (OtherBodyIndex :type Integer) (bFromSweep :type Boolean) (SweepResult :type Hit%20Result%20Structure%20%28by%20ref%29))
  (bind _asbp_player (Utilities|Casting|CastToBP_Player OtherActor))
  (if (Class|PrimitiveComponent|IsOverlappingComponent (Variables|/Game/Code/Player/BP_Player.BP_Player_C|GetDPS_AttackZone _asbp_player) OverlappedComponent)
    (Utilities|FlowControl|DoOnce false
      (:Completed
        (Variables|Default|SetisActive true)
        (Default|CallActivateSwitch)
        (Rendering|Material|SetMaterial (Variables|Default|GetCone1) 0 "/Game/Code/Puzzles/Materials/MAT_On_Simple.MAT_On_Simple")
        (Utilities|FlowControl|Delay 0.5)))))

(event EventBeginPlay
  (Variables|Default|SetInitialPosition (Variables|/Script/Engine.SceneComponent|GetRelativeLocation (Variables|Default|GetCone1)))
  (bind _newtrack_0 (Timeline|Timeline_2 Play)
    (:Update
      (Transformation|SetRelativeLocation (Variables|Default|GetCone1) (Math|Vector|Lerp(Vector) (Variables|Default|GetInitialPosition) (Variables|Default|GetEndPosition) _newtrack_0) false false))))

(fn ConstructionScript)