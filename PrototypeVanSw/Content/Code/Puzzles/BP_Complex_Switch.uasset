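; BP_Complex_Switch is a timed puzzle switch triggered when the player overlaps it.
; It sets Ready, broadcasts it, lights the handle, shows linked Barriers with collision and rotates the handle via a timeline.
; After SwitchDelay it clears Ready; unless Activate is set, a second timeline returns the handle, then the material and barriers switch off.
; A DoOnce blocks retriggering until that reset completes.
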(event EventBeginPlay
  (Transformation|SetRelativeRotation (Variables|Default|GetHandle) (Variables|Default|GetInitial_rotator) false false))

(event Collision|EventActorBeginOverlap
  (params (OtherActor :type Actor%20Object%20Reference))
  (if (Utilities|ClassIsChildOf (Utilities|GetClass OtherActor) "/Game/Code/Player/BP_Player.BP_Player_C")
    (Utilities|FlowControl|DoOnce (Variables|Default|GetActivate?) :!label _label
      (:Completed
        (Variables|Default|SetReady? true)
        (Default|CallReady)
        (Rendering|Material|SetMaterial (Variables|Default|GetHandle) 0 "/Game/Code/Puzzles/Materials/MAT_On.MAT_On")
        (for _array_element (Variables|CONFIG|GetBarriers)
          (Rendering|SetVisibility (Variables|/Game/Code/Puzzles/BP_Complex_Fence_Barrier.BP_Complex_Fence_Barrier_C|GetStaticMesh _array_element) true false)
          (Collision|SetCollisionEnabled (Variables|/Game/Code/Puzzles/BP_Complex_Fence_Barrier.BP_Complex_Fence_Barrier_C|GetStaticMesh _array_element) "QueryAndPhysics"))
        (bind _newtrack_0 (Timeline|Timeline_0 PlayFromStart)
          (:Update
            (Transformation|SetRelativeRotation (Variables|Default|GetHandle) (Math|Interpolation|Ease "Linear" _newtrack_0 (Variables|Default|GetInitial_rotator) (Variables|Default|GetEnd_rotator) true) false false))
          (:Finished
            (Utilities|FlowControl|Delay (Variables|CONFIG|GetSwitch_Delay))
            (Variables|Default|SetReady? false)
            (if (not (Variables|Default|GetActivate?))
              (bind _newtrack_0_2 (Timeline|Timeline_1 PlayFromStart)
                (:Update
                  (Transformation|SetRelativeRotation (Variables|Default|GetHandle) (Math|Interpolation|Ease "Linear" _newtrack_0_2 (Variables|Default|GetEnd_rotator) (Variables|Default|GetInitial_rotator) true) false false))
                (:Finished
                  (Rendering|Material|SetMaterial (Variables|Default|GetHandle) 0 "/Game/Code/Puzzles/Materials/MAT_Off.MAT_Off")
                  (for _array_element_2 (Variables|CONFIG|GetBarriers)
                    (Rendering|SetVisibility (Variables|/Game/Code/Puzzles/BP_Complex_Fence_Barrier.BP_Complex_Fence_Barrier_C|GetStaticMesh _array_element_2) false false)
                    (Collision|SetCollisionEnabled (Variables|/Game/Code/Puzzles/BP_Complex_Fence_Barrier.BP_Complex_Fence_Barrier_C|GetStaticMesh _array_element_2) "NoCollision"))
                  (goto _label Reset))))))))))

(fn ConstructionScript)