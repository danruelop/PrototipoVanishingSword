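; A two-player box trigger that fires only when both the male and female player characters stand inside it.
; Begin and end overlap events maintain a presence flag for each character.
; Once both flags are set, it activates spawns, closes every fence in BarriersToClose, plays the hourglass sound in 2D and destroys itself, so it fires once.
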(event EventBeginPlay
  (|CallParentFunction) ; This node is disabled and will not be called.\nDrag off pins to build functionality.
)

(event Collision|EventActorEndOverlap
  (params (OtherActor :type Actor%20Object%20Reference))
  (Utilities|Casting|CastToBP_MalePlayer OtherActor
    (:then
      (Variables|Default|SetMPlayerOverlapping false))
    (:CastFailed
      (Utilities|Casting|CastToBP_FemalePlayer OtherActor)
      (Variables|Default|SetFPlayerOverlapping false))))

(event EventTick
  (params (DeltaSeconds :type Float%20%28single-precision%29))
  (|CallParentFunction DeltaSeconds) ; This node is disabled and will not be called.\nDrag off pins to build functionality.
)

(event Collision|EventActorBeginOverlap
  (params (OtherActor :type Actor%20Object%20Reference))
  (Utilities|Casting|CastToBP_MalePlayer OtherActor
    (:then
      (Variables|Default|SetMPlayerOverlapping true))
    (:CastFailed
      (Utilities|Casting|CastToBP_FemalePlayer OtherActor)
      (Variables|Default|SetFPlayerOverlapping true)))
  (if (and (Variables|Default|GetMPlayerOverlapping) (Variables|Default|GetFPlayerOverlapping))
    (CallFunction|ActivateSpawns)
    (for _array_element (Variables|Default|GetBarriersToClose)
      (Default|CloseFenceEvent _array_element))
    (Audio|PlaySound2D "/Game/Sound/SFX/LEVEL/HOURGLASS.HOURGLASS" 1.0 1.0 0.0 0 0)
    (Actor|DestroyActor)))

(fn ConstructionScript
  (|CallParentFunction))