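; BP_ComplexDoor is a puzzle door that opens once every switch in its Switches array is active.
; On BeginPlay it binds to each switch's Ready event, which triggers a recount of consecutive active switches that stops at the first inactive one.
; When all are active, it flags each switch as DoorOpen, applies an "on" material to its HourglassClock, and hides both door halves and disables their collision.
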(event Custom|Ready_Event_1
  (bind _l_door (Variables|Default|GetL_Door))
  (bind _switches (Variables|CONFIG|GetSwitches))
  (bind _array_element (Utilities|Array|ForEachLoopwithBreak _switches :!label _label)
    (:LoopBody
      (if (Variables|/Game/Code/Puzzles/BP_HourGlass_Switch.BP_HourGlass_Switch_C|GetisActivate _array_element)
        (Variables|Default|Setindex (+ (Variables|Default|Getindex) 1))
        (else
          (goto _label Break))))
    (:Completed
      (if (== (Utilities|Array|Length _switches) (Variables|Default|Getindex))
        (for _array_element_2 (Variables|CONFIG|GetSwitches)
          (Variables|/Game/Code/Puzzles/BP_HourGlass_Switch.BP_HourGlass_Switch_C|SetdoorOpen _array_element_2 true)
          (Rendering|Material|CreateDynamicMaterialInstance (Variables|/Game/Code/Puzzles/BP_HourGlass_Switch.BP_HourGlass_Switch_C|GetHourglass_Clock _array_element_2) 0 "/Game/Code/Puzzles/Materials/MAT_On_Simple.MAT_On_Simple" "None" :!class /Script/Engine.PrimitiveComponent))
        (Rendering|SetVisibility _l_door false true)
        (Collision|SetCollisionEnabled _l_door "NoCollision")
        (else
          (Variables|Default|Setindex 0))))))

(event EventBeginPlay
  (for _array_element (Variables|CONFIG|GetSwitches)
    (EventDispatchers|AssignReady _array_element (delegate Custom|Ready_Event_1))))

(fn ConstructionScript)