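; Puzzle bridge that lowers in five screw-like steps as the player attacks its screw collider.
; An overlap with the player's DPSAttackZone selects a stage by HitLevel, each guarded by DoOnce.
; Each stage's timeline turns both pillars a quarter turn, drops the bridge mesh and fades out a sound spawned at world origin.
; HitLevel advances only when the timeline finishes, so hits during movement are ignored.
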(event OnComponentBeginOverlap(ScrewCollider)
  (params (OverlappedComponent :type Primitive%20Component%20Object%20Reference) (OtherActor :type Actor%20Object%20Reference) (OtherComp :type Primitive%20Component%20Object%20Reference) (OtherBodyIndex :type Integer) (bFromSweep :type Boolean) (SweepResult :type Hit%20Result%20Structure%20%28by%20ref%29))
  (bind _asbp_player (Utilities|Casting|CastToBP_Player OtherActor))
  (if (== (Variables|/Game/Code/Player/BP_Player.BP_Player_C|GetDPS_AttackZone _asbp_player) OtherComp)
    (switch int (Variables|Default|GethitLevel)
      (:0
        (Utilities|FlowControl|DoOnce false
          (:Completed
            (CallFunction|PlaySound)
            (bind _newtrack_0 (Timeline|Timeline_0 PlayFromStart)
              (:Update
                (Audio|Components|Audio|SetVolumeMultiplier (Variables|Default|GetSound) (Math|Float|Lerp 0.7 0.0 _newtrack_0) :!class /Script/Engine.AudioComponent)
                (Transformation|SetRelativeRotation (Variables|Default|GetPilarFront) (Math|Rotator|Lerp(Rotator) "0, 0, 0" "0,90.000000, 0" _newtrack_0) false false)
                (Transformation|SetRelativeLocation (Variables|Default|GetSM_Bridge) (Math|Vector|Lerp(Vector) "0, 0, 0" "0, 0,-87.000000" _newtrack_0) false false))
              (:Finished
                (Audio|Components|Audio|Stop (Variables|Default|GetSound))
                (Variables|Default|SethitLevel 1))))))
      (:1
        (Utilities|FlowControl|DoOnce false
          (:Completed
            (CallFunction|PlaySound)
            (bind _newtrack_0_2 (Timeline|Timeline_1 PlayFromStart)
              (:Update
                (Audio|Components|Audio|SetVolumeMultiplier (Variables|Default|GetSound) (Math|Float|Lerp 0.7 0.0 _newtrack_0_2) :!class /Script/Engine.AudioComponent)
                (Transformation|SetRelativeRotation (Variables|Default|GetPilarFront) (Math|Rotator|Lerp(Rotator) "0,90.000000, 0" "0,180.000000, 0" _newtrack_0_2) false false)
                (Transformation|SetRelativeLocation (Variables|Default|GetSM_Bridge) (Math|Vector|Lerp(Vector) "0, 0,-87.000000" "0, 0,-174.000000" _newtrack_0_2) false false))
              (:Finished
                (Audio|Components|Audio|Stop (Variables|Default|GetSound))
                (Variables|Default|SethitLevel 2))))))
      (:2
        (Utilities|FlowControl|DoOnce false
          (:Completed
            (CallFunction|PlaySound)
            (bind _newtrack_0_3 (Timeline|Timeline_2 PlayFromStart)
              (:Update
                (Audio|Components|Audio|SetVolumeMultiplier (Variables|Default|GetSound) (Math|Float|Lerp 0.7 0.0 _newtrack_0_3) :!class /Script/Engine.AudioComponent)
                (Transformation|SetRelativeRotation (Variables|Default|GetPilarFront) (Math|Rotator|Lerp(Rotator) "0,180.000000, 0" "0,270.000000, 0" _newtrack_0_3) false false)
                (Transformation|SetRelativeLocation (Variables|Default|GetSM_Bridge) (Math|Vector|Lerp(Vector) "0, 0,-174.000000" "0, 0,-261.000000" _newtrack_0_3) false false))
              (:Finished
                (Audio|Components|Audio|Stop (Variables|Default|GetSound))
                (Variables|Default|SethitLevel 3))))))
      (:3
        (Utilities|FlowControl|DoOnce false
          (:Completed
            (CallFunction|PlaySound)
            (bind _newtrack_0_4 (Timeline|Timeline_3 PlayFromStart)
              (:Update
                (Audio|Components|Audio|SetVolumeMultiplier (Variables|Default|GetSound) (Math|Float|Lerp 0.7 0.0 _newtrack_0_4) :!class /Script/Engine.AudioComponent)
                (Transformation|SetRelativeRotation (Variables|Default|GetPilarFront) (Math|Rotator|Lerp(Rotator) "0,270.000000, 0" "0,360.000000, 0" _newtrack_0_4) false false)
                (Transformation|SetRelativeLocation (Variables|Default|GetSM_Bridge) (Math|Vector|Lerp(Vector) "0, 0,-261.000000" "0, 0,-348.000000" _newtrack_0_4) false false))
              (:Finished
                (Audio|Components|Audio|Stop (Variables|Default|GetSound))
                (Variables|Default|SethitLevel 4))))))
      (:4
        (Utilities|FlowControl|DoOnce false
          (:Completed
            (CallFunction|PlaySound)
            (bind _newtrack_0_5 (Timeline|Timeline_4 PlayFromStart)
              (:Update
                (Audio|Components|Audio|SetVolumeMultiplier (Variables|Default|GetSound) (Math|Float|Lerp 0.7 0.0 _newtrack_0_5) :!class /Script/Engine.AudioComponent)
                (Transformation|SetRelativeRotation (Variables|Default|GetPilarFront) (Math|Rotator|Lerp(Rotator) "0,360.000000, 0" "0,450.000000, 0" _newtrack_0_5) false false)
                (Transformation|SetRelativeLocation (Variables|Default|GetSM_Bridge) (Math|Vector|Lerp(Vector) "0, 0,-348.000000" "0, 0,-435.000000" _newtrack_0_5) false false))
              (:Finished
                (Audio|Components|Audio|Stop (Variables|Default|GetSound))
                (Variables|Default|SethitLevel 5)))))))))

(event Custom|PlaySound
  (bind _returnvalue (Audio|SpawnSoundatLocation "/Game/Sound/SFX/LEVEL/BRIDGE.BRIDGE" "0, 0, 0" "0, 0, 0" 1.0 1.0 0.0 0 0))
  (Variables|Default|SetSound _returnvalue))

(fn ConstructionScript)