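; Timed hourglass puzzle switch, triggered when a player's melee attack zone overlaps its box, that closes linked fence barriers until it expires.
; Activation calls Ready, then chained timelines flip the box, drive the material's Interpolator over SwitchDelay, then flip back as barriers reopen and the switch rearms.
; If DoorOpen is set at a stage check, it stays active with a solid "on" material and stencil highlight.
; Start and end sounds accompany the countdown.
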(event OnComponentBeginOverlap(Box)
  (params (OverlappedComponent :type Primitive%20Component%20Object%20Reference) (OtherActor :type Actor%20Object%20Reference) (OtherComp :type Primitive%20Component%20Object%20Reference) (OtherBodyIndex :type Integer) (bFromSweep :type Boolean) (SweepResult :type Hit%20Result%20Structure%20%28by%20ref%29))
  (bind _asbp_player (Utilities|Casting|CastToBP_Player OtherActor))
  (if (Math|Boolean|ORBoolean (== (Variables|/Game/Code/Player/BP_Player.BP_Player_C|GetDPS_AttackZoneSlash _asbp_player) OtherComp) (== (Variables|/Game/Code/Player/BP_Player.BP_Player_C|GetDPS_AttackZoneSlash2 _asbp_player) OtherComp) (== (Variables|/Game/Code/Player/BP_Player.BP_Player_C|GetDPS_AttackZoneUppercut _asbp_player) OtherComp))
    (if (not (Variables|Components|GetisActivate))
      (Variables|Components|SetisActivate true)
      (Default|CallReady)
      (if (Variables|Components|GetdoorOpen)
        (Utilities|FlowControl|DoOnce false
          (:Completed
            (Rendering|Material|CreateDynamicMaterialInstance (Variables|Default|GetHourglass_Clock) 0 "/Game/Code/Puzzles/Materials/MAT_On_Simple.MAT_On_Simple" "None" :!class /Script/Engine.PrimitiveComponent)
            (Rendering|SetCustomDepthStencilValue (Variables|Default|GetHourglass_Base) 6)
            (CallFunction|PlaysOUND)
            (for _array_element (Variables|CONFIG|GetBarriers)
              (Default|CloseFenceEvent _array_element))))
        (else
          (bind _returnvalue (Rendering|Material|CreateDynamicMaterialInstance (Variables|Default|GetHourglass_Clock) 0 "/Game/Code/Puzzles/Materials/MAT_Running_Hourglass.MAT_Running_Hourglass" "None" :!class /Script/Engine.PrimitiveComponent))
          (Rendering|SetCustomDepthStencilValue (Variables|Default|GetHourglass_Base) 5)
          (CallFunction|PlaysOUND)
          (for _array_element_2 (Variables|CONFIG|GetBarriers)
            (Default|CloseFenceEvent _array_element_2))
          (bind _newtrack_0 (Timeline|Timeline_0 PlayFromStart)
            (:Update
              (Rendering|Material|SetScalarParameterValue _returnvalue "Interpolator" (Math|Float|Lerp 0.0 1.0 _newtrack_0) :!class /Script/Engine.MaterialInstanceDynamic)
              (Transformation|SetRelativeRotation (Variables|Default|GetBox) (Math|Rotator|Lerp(Rotator) "0, 0, 0" "0.000000,0.000000,180.000000" _newtrack_0) false false))
            (:Finished
              (if (Variables|Components|GetdoorOpen)
                (Utilities|FlowControl|DoOnce false
                  (:Completed
                    (Rendering|SetCustomDepthStencilValue (Variables|Default|GetHourglass_Base) 6)
                    (Rendering|Material|CreateDynamicMaterialInstance (Variables|Default|GetHourglass_Clock) 0 "/Game/Code/Puzzles/Materials/MAT_On_Simple.MAT_On_Simple" "None" :!class /Script/Engine.PrimitiveComponent)))
                (else
                  (Components|Timeline|SetPlayRate (Variables|Default|GetTimeline_3) (/ 1.0 (Variables|CONFIG|GetSwitchDelay)))
                  (bind _newtrack_0_2 (Timeline|Timeline_3 PlayFromStart)
                    (:Update
                      (Rendering|Material|SetScalarParameterValue _returnvalue "Interpolator" _newtrack_0_2 :!class /Script/Engine.MaterialInstanceDynamic))
                    (:Finished
                      (if (Variables|Components|GetdoorOpen)
                        (Utilities|FlowControl|DoOnce false
                          (:Completed
                            (Rendering|SetCustomDepthStencilValue (Variables|Default|GetHourglass_Base) 6)
                            (Rendering|Material|CreateDynamicMaterialInstance (Variables|Default|GetHourglass_Clock) 0 "/Game/Code/Puzzles/Materials/MAT_On_Simple.MAT_On_Simple" "None" :!class /Script/Engine.PrimitiveComponent)))
                        (else
                          (CallFunction|PlayEnd)
                          (for _array_element_3 (Variables|CONFIG|GetBarriers)
                            (Default|OpenFenceEvent _array_element_3))
                          (bind _newtrack_0_3 (Timeline|Timeline_1 PlayFromStart)
                            (:Update
                              (Rendering|Material|SetScalarParameterValue _returnvalue "Interpolator" (Math|Float|Lerp 1.0 0.0 _newtrack_0_3) :!class /Script/Engine.MaterialInstanceDynamic)
                              (Transformation|SetRelativeRotation (Variables|Default|GetBox) (Math|Rotator|Lerp(Rotator) "0.000000, 0,180.000000" "0, 0, 0" _newtrack_0_3) false false))
                            (:Finished
                              (if (Variables|Components|GetdoorOpen)
                                (Utilities|FlowControl|DoOnce false
                                  (:Completed
                                    (Rendering|SetCustomDepthStencilValue (Variables|Default|GetHourglass_Base) 6)
                                    (Rendering|Material|CreateDynamicMaterialInstance (Variables|Default|GetHourglass_Clock) 0 "/Game/Code/Puzzles/Materials/MAT_On_Simple.MAT_On_Simple" "None" :!class /Script/Engine.PrimitiveComponent)))
                                (else
                                  (Variables|Components|SetisActivate false))))))))))))))))))

(event Custom|PlaySound
  (Audio|Components|Audio|Play (Variables|Default|GetHourGlassStart) 0.0)
  (Components|Timeline|SetPlayRate (Variables|Default|GetTimeline_2) (/ 1.0 (Variables|CONFIG|GetSwitchDelay)))
  (bind _newtrack_0 (Timeline|Timeline_2 PlayFromStart)
    (:Update
      (Audio|Components|Audio|SetVolumeMultiplier (Variables|Default|GetHourGlassStart) (Math|Float|Lerp 0.6 0.3 _newtrack_0) :!class /Script/Engine.AudioComponent))))

(event Custom|PlayEnd
  (bind _hourglassend (Variables|Default|GetHourGlassEnd))
  (Audio|Components|Audio|FadeIn _hourglassend 1.0 0.7 8.0 "Linear" :!class /Script/Engine.AudioComponent)
  (Audio|Components|Audio|FadeOut _hourglassend 1.0 0.7 "Linear" :!class /Script/Engine.AudioComponent))

(event EventBeginPlay
  (bind _returnvalue (AddComponent|AddAudioComponent false))
  (Variables|Default|SetHourGlassStart _returnvalue)
  (bind _returnvalue_2 (AddComponent|AddAudioComponent false))
  (Variables|Default|SetHourGlassEnd _returnvalue_2))

(fn ConstructionScript)