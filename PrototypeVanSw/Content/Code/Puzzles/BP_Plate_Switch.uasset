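; Two-player co-op pressure plate switch that needs the male player on the blue plate and the female player on the orange plate simultaneously.
; Overlap events light each plate for its matching character and turn it off on exit until solved.
; Both begin-overlap events share an occupancy check that, once satisfied, latches both plates on through BActivate, calls EDOpen and activates spawns.
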(event OnComponentEndOverlap(PlatformBlue)
  (params (OverlappedComponent :type Primitive%20Component%20Object%20Reference) (OtherActor :type Actor%20Object%20Reference) (OtherComp :type Primitive%20Component%20Object%20Reference) (OtherBodyIndex :type Integer))
  (if (not (Variables|Default|GetB_Activate?))
    (if (Utilities|ClassIsChildOf (Utilities|GetClass OtherActor) "/Game/Code/Player/BP_MalePlayer.BP_MalePlayer_C")
      (Rendering|Material|SetMaterial (Variables|Default|GetPlatformBlue) 0 "/Game/Code/Puzzles/Materials/MAT_Off.MAT_Off"))))

(event OnComponentBeginOverlap(PlatformOrange)
  (params (OverlappedComponent :type Primitive%20Component%20Object%20Reference) (OtherActor :type Actor%20Object%20Reference) (OtherComp :type Primitive%20Component%20Object%20Reference) (OtherBodyIndex :type Integer) (bFromSweep :type Boolean) (SweepResult :type Hit%20Result%20Structure%20%28by%20ref%29))
  (if (not (Variables|Default|GetB_Activate?))
    (if (Utilities|ClassIsChildOf (Utilities|GetClass OtherActor) "/Game/Code/Player/BP_FemalePlayer.BP_FemalePlayer_C")
      (Rendering|Material|SetMaterial (Variables|Default|GetPlatformOrange) 0 "/Game/Code/Puzzles/Materials/MAT_On_Orange_Plessure.MAT_On_Orange_Plessure")
      (if (and (>= (Utilities|Array|Length (Collision|GetOverlappingActors (Variables|Default|GetPlatformBlue) "/Game/Code/Player/BP_MalePlayer.BP_MalePlayer_C" :!class /Script/Engine.PrimitiveComponent)) 1) (>= (Utilities|Array|Length (Collision|GetOverlappingActors (Variables|Default|GetPlatformOrange) "/Game/Code/Player/BP_FemalePlayer.BP_FemalePlayer_C" :!class /Script/Engine.PrimitiveComponent)) 1))
        (Utilities|FlowControl|DoOnce false
          (:Completed
            (Rendering|Material|SetMaterial (Variables|Default|GetPlatformBlue) 0 "/Game/Code/Puzzles/Materials/MAT_On.MAT_On")
            (Variables|Default|SetB_Activate? true)
            (Default|CallEDOpen)
            (CallFunction|ActivateSpawns)))))))

(event OnComponentEndOverlap(PlatformOrange)
  (params (OverlappedComponent :type Primitive%20Component%20Object%20Reference) (OtherActor :type Actor%20Object%20Reference) (OtherComp :type Primitive%20Component%20Object%20Reference) (OtherBodyIndex :type Integer))
  (if (not (Variables|Default|GetB_Activate?))
    (if (Utilities|ClassIsChildOf (Utilities|GetClass OtherActor) "/Game/Code/Player/BP_FemalePlayer.BP_FemalePlayer_C")
      (Rendering|Material|SetMaterial (Variables|Default|GetPlatformOrange) 0 "/Game/Code/Puzzles/Materials/MAT_Off.MAT_Off"))))

(event OnComponentBeginOverlap(PlatformBlue)
  (params (OverlappedComponent :type Primitive%20Component%20Object%20Reference) (OtherActor :type Actor%20Object%20Reference) (OtherComp :type Primitive%20Component%20Object%20Reference) (OtherBodyIndex :type Integer) (bFromSweep :type Boolean) (SweepResult :type Hit%20Result%20Structure%20%28by%20ref%29))
  (if (not (Variables|Default|GetB_Activate?))
    (if (Utilities|ClassIsChildOf (Utilities|GetClass OtherActor) "/Game/Code/Player/BP_MalePlayer.BP_MalePlayer_C")
      (Rendering|Material|SetMaterial (Variables|Default|GetPlatformBlue) 0 "/Game/Code/Puzzles/Materials/MAT_On_Blue_Plessure.MAT_On_Blue_Plessure")
      (if (and (>= (Utilities|Array|Length (Collision|GetOverlappingActors (Variables|Default|GetPlatformBlue) "/Game/Code/Player/BP_MalePlayer.BP_MalePlayer_C" :!class /Script/Engine.PrimitiveComponent)) 1) (>= (Utilities|Array|Length (Collision|GetOverlappingActors (Variables|Default|GetPlatformOrange) "/Game/Code/Player/BP_FemalePlayer.BP_FemalePlayer_C" :!class /Script/Engine.PrimitiveComponent)) 1))
        (Utilities|FlowControl|DoOnce false
          (:Completed
            (Rendering|Material|SetMaterial (Variables|Default|GetPlatformBlue) 0 "/Game/Code/Puzzles/Materials/MAT_On.MAT_On")
            (Variables|Default|SetB_Activate? true)
            (Default|CallEDOpen)
            (CallFunction|ActivateSpawns)))))))

(fn ConstructionScript)