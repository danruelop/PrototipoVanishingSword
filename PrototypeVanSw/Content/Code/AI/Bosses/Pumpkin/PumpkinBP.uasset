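; Pumpkin boss Blueprint that attacks players, takes damage and ends the game when its health runs out.
; On BeginPlay it spawns a shield on its right arm socket and swaps hit collision from the body capsule to the back capsule.
; HitPlayer and HitArea damage every player within normal or charged attack range through the UI master, which also receives the end-game message.
; Damage and stun events include debug prints.
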(event Custom|ActivateDefaultCapsule
  (params (Active :type Boolean))
  (bind _bodycapsule (Variables|Default|GetBodyCapsule))
  (if Active
    (Collision|SetCollisionEnabled _bodycapsule "QueryOnly")
    (Components|Activation|Activate _bodycapsule false)
    (else
      (Collision|SetCollisionEnabled _bodycapsule "NoCollision")
      (Components|Activation|Deactivate _bodycapsule))))

(event EventBeginPlay
  (bind _backcapsule (Variables|Default|GetBackCapsule))
  (bind _returnvalue (Game|SpawnActorfromClass "/Game/Code/AI/Bosses/Pumpkin/ShieldBP.ShieldBP_C" (Math|Transform|MakeTransform "0.000000,0.000000,150.000000" "25.000000,120.000000,40.000000" "0.750000,0.750000,1") "AlwaysSpawn" 0 0))
  (Transformation|AttachComponentToComponent _returnvalue (Variables|Character|GetMesh) "RightArm" "KeepRelative" "KeepRelative" "KeepRelative" true)
  (CallFunction|ActivateDefaultCapsule false)
  (Collision|SetCollisionEnabled _backcapsule "QueryOnly")
  (Components|Activation|Activate _backcapsule false))

(event EventHitPlayer
  (bind _outactors (Actor|GetAllActorsOfClass "/Game/Code/Player/BP_Player.BP_Player_C"))
  (for _array_element _outactors
    (if (< (Transformation|GetDistanceTo _array_element self) (Variables|Default|GetAttackRange))
      (bind _returnvalue (Actor|GetActorOfClass "/Game/UI/UI_Code/BP_UI_Master.BP_UI_Master_C"))
      (Class|BPIonHit|PlayerReceivesDamage(Message) _returnvalue (Variables|/Game/Code/Player/BP_Player.BP_Player_C|GetiPlayerIndex _array_element) (Variables|Default|GetfDamage))
      (Development|PrintString (Utilities|String|Append "HIT  " (Utilities|GetObjectName (Variables|Default|GetTarget)))))))

(event EventApplyDamage
  (params (DPSBasicAttackDamage :type Integer))
  (Class|Enemy|Damage DPSBasicAttackDamage)
  (Development|PrintString (Utilities|String|Append "Boss HEALTH: " (Utilities|String|ToString(Integer) (Variables|Default|GetHealth))))
  ;[1 1 1] When dead end game
  (if (<= (Variables|Default|GetHealth) 0)
    (bind _returnvalue (Actor|GetActorOfClass "/Game/UI/UI_Code/BP_UI_Master.BP_UI_Master_C"))
    (Class|BPIonHit|EndGame(Message) _returnvalue)))

(event EventHitArea
  (bind _outactors (Actor|GetAllActorsOfClass "/Game/Code/Player/BP_Player.BP_Player_C"))
  (for _array_element _outactors
    (if (< (Transformation|GetDistanceTo _array_element self) (Variables|Default|GetAttackChargedRange))
      (bind _returnvalue (Actor|GetActorOfClass "/Game/UI/UI_Code/BP_UI_Master.BP_UI_Master_C"))
      (Class|BPIonHit|PlayerReceivesDamage(Message) _returnvalue (Variables|/Game/Code/Player/BP_Player.BP_Player_C|GetiPlayerIndex _array_element) (Variables|Default|GetfDamage))
      (Development|PrintString (Utilities|String|Append "HIT  " (Utilities|GetObjectName _array_element))))))

(event EventApplyStun
  (Class|ZombieEnemy|Stun)
  (Development|PrintString "Me stuneaste >:("))

(fn ConstructionScript)