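; Pumpkin boss that hurts players with a shield attack and ends the game when it dies.
; The shield damage box attaches to the right hand, toggles collision through enable/disable functions, and reports overlap damage to BP_UI_Master.
; Damage and stun events set state flags that cancel attacks, while timers gate area attacks.
; Once DeathFadingOut is set, Tick sinks the actor below a height threshold, destroys it and sends the end-game message.
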(event OnComponentBeginOverlap(ShieldDamageBox)
  (params (OverlappedComponent :type Primitive%20Component%20Object%20Reference) (OtherActor :type Actor%20Object%20Reference) (OtherComp :type Primitive%20Component%20Object%20Reference) (OtherBodyIndex :type Integer) (bFromSweep :type Boolean) (SweepResult :type Hit%20Result%20Structure%20%28by%20ref%29))
  ;[1 1 1] Hurt Player with Basic Attack
  (bind _asbp_player (Utilities|Casting|CastToBP_Player OtherActor))
  (CallFunction|HurtPlayer _asbp_player (Variables|Default|GetSimpleAttackDamage))
  (Variables|Default|SetTimeSinceLastDamage 0.0))

(event EventBeginPlay
  ;[1 1 1] Attach Shield
  (Transformation|AttachComponentToComponent (Variables|Default|GetShieldDamageBox) (Variables|Character|GetMesh) "RightHand" "KeepRelative" "KeepRelative" "KeepRelative" true)
  (CallFunction|DisableShieldDamageCapsule)
  ;[1 1 1] Set Nest in the position wich the Actor is placed in the world
  (Variables|Default|SetNest (Transformation|GetActorLocation))
  (Variables|Default|SetTimeSinceLastAttackStart 0.0)
  (Variables|Default|SetTimeSinceLastDamage 0.0))

(event EventTick
  (params (DeltaSeconds :type Float%20%28single-precision%29))
  (Variables|Default|SetTimeSinceLastAttackStart (+ (Variables|Default|GetTimeSinceLastAttackStart) DeltaSeconds))
  (Variables|Default|SetTimeSinceLastDamage (+ (Variables|Default|GetTimeSinceLastDamage) DeltaSeconds))
  ;[1 1 1] Death fade out (when dead anim ends)
  (if (Variables|Default|GetDeathFadingOut)
    (Collision|SetCollisionEnabled (Variables|Default|GetCapsuleComponent) "NoCollision")
    (Transformation|AddActorLocalOffset (* (Math|Vector|MakeVector 0.0 0.0 -5e+01) DeltaSeconds) false false)
    (if (< (.Z (Math|Vector|BreakVector (Transformation|GetActorLocation))) 5e+02)
      (Actor|DestroyActor)
      ;[1 1 1] End game
      (bind _returnvalue (Actor|GetActorOfClass "/Game/UI/UI_Code/BP_UI_Master.BP_UI_Master_C"))
      (Class|BPIonHit|EndGame(Message) _returnvalue))))

(event EventApplyDamage
  (params (DPSBasicAttackDamage :type Integer))
  ;[1 1 1] Receive damage
  (Variables|Default|SetHealth (- (Variables|Default|GetHealth) DPSBasicAttackDamage))
  (Variables|Default|SetHitReceived true)
  (Variables|Default|SetReactingToHit true)
  (Variables|Default|SetAttacking false)
  (Variables|Default|SetAttackingInArea false))

(event EventApplyStun
  ;[1 1 1] Receive stun
  (Variables|Default|SetStunReceived true)
  (Variables|Default|SetStunned true)
  (Variables|Default|SetAttacking false)
  (Variables|Default|SetAttackingInArea false))

(fn ConstructionScript)

(fn EnableShieldDamageCapsule
  (Collision|SetCollisionEnabled (Variables|Default|GetShieldDamageBox) "QueryOnly"))

(fn DisableShieldDamageCapsule
  (Collision|SetCollisionEnabled (Variables|Default|GetShieldDamageBox) "NoCollision"))

(fn AttackinArea
  (bind _able (CallFunction|IsTimeAbletoAttack))
  (if _able
    (Variables|Default|SetAttackingInArea true)
    (Variables|Default|SetTimeSinceLastAttackStart 0.0)))

(fn HurtPlayer
  (params (Player :type BP%20Player%20Object%20Reference) (Damage :type Float%20%28single-precision%29))
  (if (> (Variables|Default|GetTimeSinceLastDamage) 0.0)
    (bind _returnvalue (Actor|GetActorOfClass "/Game/UI/UI_Code/BP_UI_Master.BP_UI_Master_C"))
    (Class|BPIonHit|PlayerReceivesDamage(Message) _returnvalue (Variables|/Game/Code/Player/BP_Player.BP_Player_C|GetiPlayerIndex Player) Damage)))