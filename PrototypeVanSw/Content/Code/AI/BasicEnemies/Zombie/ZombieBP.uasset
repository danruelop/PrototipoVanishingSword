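; Blueprint for a basic zombie enemy that damages nearby players and reacts to incoming damage and stuns.
; HitPlayer checks every BP_Player against AttackRange and reports damage for those in range, by player index, to the BP_UI_Master actor.
; ApplyDamage and ApplyStun forward to Damage and Stun functions defined outside this graph, with debug prints on hits, health and stuns.
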(event EventHitPlayer
  (bind _outactors (Actor|GetAllActorsOfClass "/Game/Code/Player/BP_Player.BP_Player_C"))
  (for _array_element _outactors
    (if (< (Transformation|GetDistanceTo _array_element self) (Variables|Default|GetAttackRange))
      (bind _returnvalue (Actor|GetActorOfClass "/Game/UI/UI_Code/BP_UI_Master.BP_UI_Master_C"))
      (Class|BPIonHit|PlayerReceivesDamage(Message) _returnvalue (Variables|/Game/Code/Player/BP_Player.BP_Player_C|GetiPlayerIndex _array_element) (Variables|Default|GetfDamage))
      (Development|PrintString (Utilities|String|Append "HIT  " (Utilities|GetObjectName (Variables|Default|GetTarget)))))))

(event EventApplyStun
  (Class|ZombieEnemy|Stun)
  (Development|PrintString "Me stuneaste >:("))

(event EventApplyDamage
  (params (DPSBasicAttackDamage :type Integer))
  (Class|Enemy|Damage DPSBasicAttackDamage)
  (Development|PrintString (Utilities|String|Append "Zombie HEALTH: " (Utilities|String|ToString(Integer) (Variables|Default|GetHealth)))))

(fn ConstructionScript)