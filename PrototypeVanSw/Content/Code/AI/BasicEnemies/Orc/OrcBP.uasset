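; Orc enemy Blueprint that takes damage and stuns and reports hand hits to the player UI.
; A collision capsule on the RightHand socket, toggled by enable/disable functions, messages BP_UI_Master on player overlap, currently with zero damage.
; Incoming damage and stun events set state flags and cancel attacking.
; Tick advances attack and damage timers and, while DeathFadingOut, sinks the collisionless body until destroyed below a fixed world height.
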(event OnComponentBeginOverlap(HandDamageCapsule)
  (params (OverlappedComponent :type Primitive%20Component%20Object%20Reference) (OtherActor :type Actor%20Object%20Reference) (OtherComp :type Primitive%20Component%20Object%20Reference) (OtherBodyIndex :type Integer) (bFromSweep :type Boolean) (SweepResult :type Hit%20Result%20Structure%20%28by%20ref%29))
  ;[1 1 1] Hurt Player with Basic Attack
  (if (> (Variables|Default|GetTimeSinceLastDamage) 0.0)
    (bind _asbp_player (Utilities|Casting|CastToBP_Player OtherActor))
    (bind _returnvalue (Actor|GetActorOfClass "/Game/UI/UI_Code/BP_UI_Master.BP_UI_Master_C"))
    (Class|BPIonHit|PlayerReceivesDamage(Message) _returnvalue (Variables|/Game/Code/Player/BP_Player.BP_Player_C|GetiPlayerIndex _asbp_player) 0.0)
    (Variables|Default|SetTimeSinceLastDamage 0.0)))

(event EventBeginPlay
  ;[1 1 1] Attach HandDamageCapsule
  (Transformation|AttachComponentToComponent (Variables|Default|GetHandDamageCapsule) (Variables|Character|GetMesh) "RightHand" "KeepRelative" "KeepRelative" "KeepRelative" true)
  (CallFunction|DisableHandDamageCapsule)
  (Variables|Default|SetTimeSinceLastAttackStart 0.0)
  (Variables|Default|SetTimeSinceLastDamage 0.0))

(event EventTick
  (params (DeltaSeconds :type Float%20%28single-precision%29))
  (Variables|Default|SetTimeSinceLastAttackStart (+ (Variables|Default|GetTimeSinceLastAttackStart) DeltaSeconds))
  (Variables|Default|SetTimeSinceLastDamage (+ (Variables|Default|GetTimeSinceLastDamage) DeltaSeconds))
  ;[1 1 1] Death fade out (when dead anim ends)
  (if (Variables|Default|GetDeathFadingOut)
    (Collision|SetCollisionEnabled (Variables|Default|GetCapsuleComponent) "NoCollision")
    (Transformation|AddActorLocalOffset (* (Math|Vector|MakeVector 0.0 0.0 -5e+01) DeltaSeconds) false false)
    (if (< (.Z (Math|Vector|BreakVector (Transformation|GetActorLocation))) 2e+02)
      (Actor|DestroyActor))))

(event EventApplyDamage
  (params (DPSBasicAttackDamage :type Integer))
  ;[1 1 1] Receive damage
  (Variables|Default|SetHealth (- (Variables|Default|GetHealth) DPSBasicAttackDamage))
  (Variables|Default|SetHitReceived true)
  (Variables|Default|SetReactingToHit true)
  (Variables|Default|SetAttacking false))

(event EventApplyStun
  ;[1 1 1] Receive stun
  (Variables|Default|SetStunReceived true)
  (Variables|Default|SetStunned true)
  (Variables|Default|SetAttacking false))

(fn ConstructionScript)

(fn EnableHandDamageCapsule
  (Collision|SetCollisionEnabled (Variables|Default|GetHandDamageCapsule) "QueryOnly"))

(fn DisableHandDamageCapsule
  (Collision|SetCollisionEnabled (Variables|Default|GetHandDamageCapsule) "NoCollision"))