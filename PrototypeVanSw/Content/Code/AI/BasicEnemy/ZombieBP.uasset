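; Zombie enemy Blueprint with a placeholder melee hit check against third-person player characters.
; Its HitPlayer event gets every ThirdPersonCharacter in the level and compares each one's distance to the zombie against AttackRange.
; A character in range only triggers a debug "HIT" print with an object name, with no damage applied.
; The construction script is empty.
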(event EventHitPlayer
  (bind _outactors (Actor|GetAllActorsOfClass "/Game/ThirdPersonCPP/Blueprints/ThirdPersonCharacter.ThirdPersonCharacter_C"))
  (for _array_element _outactors
    (if (< (Transformation|GetDistanceTo _array_element self) (Variables|Default|GetAttackRange))
      (Development|PrintString (Utilities|String|Append "HIT  " (Utilities|GetObjectName (Variables|Default|GetTarget)))))))

(fn ConstructionScript)