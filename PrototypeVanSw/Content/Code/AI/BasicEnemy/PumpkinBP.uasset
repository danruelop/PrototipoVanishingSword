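; Pumpkin basic enemy Blueprint that carries a shield and provides normal and charged attack hit checks.
; On BeginPlay it spawns a ShieldBP and attaches it to the mesh's RightArm socket.
; HitPlayer and HitArea distance-test every ThirdPersonCharacter against AttackRange and AttackChargedRange respectively.
; Hits only print debug text without applying damage; HitPlayer names Target rather than the character found in range.
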(event EventBeginPlay
  (bind _returnvalue (Game|SpawnActorfromClass "/Game/Code/AI/BasicEnemy/ShieldBP.ShieldBP_C" (Math|Transform|MakeTransform "-50.000000,0.000000,100.000000" "0.000000,175.000000,30.000000") "AlwaysSpawn" 0 0))
  (Transformation|AttachComponentToComponent _returnvalue (Variables|Character|GetMesh) "RightArm" "KeepRelative" "KeepRelative" "KeepRelative" true))

(event EventHitPlayer
  (bind _outactors (Actor|GetAllActorsOfClass "/Game/ThirdPersonCPP/Blueprints/ThirdPersonCharacter.ThirdPersonCharacter_C"))
  (for _array_element _outactors
    (if (< (Transformation|GetDistanceTo _array_element self) (Variables|Default|GetAttackRange))
      (Development|PrintString (Utilities|String|Append "HIT  " (Utilities|GetObjectName (Variables|Default|GetTarget)))))))

(event EventHitArea
  (bind _outactors (Actor|GetAllActorsOfClass "/Game/ThirdPersonCPP/Blueprints/ThirdPersonCharacter.ThirdPersonCharacter_C"))
  (for _array_element _outactors
    (if (< (Transformation|GetDistanceTo _array_element self) (Variables|Default|GetAttackChargedRange))
      (Development|PrintString (Utilities|String|Append "HIT  " (Utilities|GetObjectName _array_element))))))

(fn ConstructionScript)