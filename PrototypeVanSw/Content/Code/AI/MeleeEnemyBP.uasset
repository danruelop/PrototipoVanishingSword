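; MeleeEnemyBP is a melee enemy character Blueprint that exposes helper functions for movement speed and timed attacks.
; SetStopVelocity and SetRunVelocity switch the CharacterMovement max walk speed between zero and the Velocity variable.
; Attack sets the Attacking flag and resets the attack timer once IsTimeAbleToAttack finds that TimeBetweenAttacks has elapsed.
; The event graph is empty, so nothing in this file advances the timer, clears the flag or calls these functions.
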(event EventBeginPlay)

(event Collision|EventActorBeginOverlap
  (params (OtherActor :type Actor%20Object%20Reference)))

(event EventTick
  (params (DeltaSeconds :type Float%20%28single-precision%29)))

(fn ConstructionScript)

(fn SetStopVelocity
  (Variables|/Script/Engine.CharacterMovementComponent|SetMaxWalkSpeed (Variables|Character|GetCharacterMovement) 0.0))

(fn SetRunVelocity
  (Variables|/Script/Engine.CharacterMovementComponent|SetMaxWalkSpeed (Variables|Character|GetCharacterMovement) (Variables|Configurable|GetVelocity)))

(fn IsTimeAbletoAttack
  (return (> (Variables|Default|GetTimeSinceLastAttackStart) (Variables|Configurable|GetTimeBetweenAttacks))))

(fn Attack
  (bind _able (CallFunction|IsTimeAbletoAttack))
  (if _able
    (Variables|Default|SetAttacking true)
    (Variables|Default|SetTimeSinceLastAttackStart 0.0)))