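; Game mode that sets up local two-player play with a male and a female character and assigns the starting DPS role.
; On BeginPlay it creates a second player controller, which possesses the level's BP_FemalePlayer, while the default controller possesses BP_MalePlayer, giving each a player index.
; It then spawns BP_Sword, snaps it to the male player's sword socket and flags him as DPS.
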(event EventBeginPlay
  (bind _returnvalue (Game|GetPlayerController 1))
  ;[1 1 1] Created a new player controller to possess the female character
  (Class|GameplayStatics|CreatePlayer 1)
  (if (!= _returnvalue 0)
    (bind _returnvalue_2 (Actor|GetActorOfClass "/Game/Code/Player/BP_FemalePlayer.BP_FemalePlayer_C"))
    (if (Utilities|IsValid _returnvalue_2)
      (Variables|/Game/Code/Player/BP_Player.BP_Player_C|SetiPlayerIndex _returnvalue_2 1)
      (Pawn|Possess _returnvalue _returnvalue_2))
    ;[1 1 1] Male player is possessed by the default player controller (0)
    (bind _returnvalue_3 (Actor|GetActorOfClass "/Game/Code/Player/BP_MalePlayer.BP_MalePlayer_C"))
    (Variables|/Game/Code/Player/BP_Player.BP_Player_C|SetiPlayerIndex _returnvalue_3 0)
    (Pawn|Possess (Game|GetPlayerController 0) _returnvalue_3)
    ;[1 1 1] Sword is created at the start of the level and is attached by default to the male player, who obtains the DPS rol (isDPS = true)
    (bind _returnvalue_4 (Game|SpawnActorfromClass "/Game/Code/Player/BP_Sword.BP_Sword_C" (Math|Conversions|ToTransform(Vector) (Transformation|GetActorForwardVector _returnvalue_3)) "Undefined" 0 0))
    (Transformation|AttachComponentToComponent _returnvalue_4 (Variables|/Game/Code/Player/BP_Player.BP_Player_C|GetSword _returnvalue_3) "SwordSocket" "SnapToTarget" "SnapToTarget" "KeepWorld" true)
    (Variables|/Game/Code/Player/BP_Player.BP_Player_C|SetbIsDPS _returnvalue_3 true)))

(fn ConstructionScript)