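; A destructible broken pillar environment actor that shatters after taking enough hits.
; Each ApplyDamage call adds to a hit counter until it reaches HitsToBreak.
; The Destructible component then takes full radial damage with an impulse at the actor's location, starts simulating physics, and the actor is flagged broken.
; The actor destroys itself after a fixed delay to clear the debris.
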(event EventApplyDamage
  (params (DPSBasicAttackDamage :type Integer))
  (if (not (Variables|Default|GetisBroken))
    (bind _output_get (Variables|Default|SetHitsCount (+ (Variables|Default|GetHitsCount) 1.0)))
    (if (>= _output_get (Variables|Default|GetHitsToBreak))
      (Class|DestructibleComponent|ApplyRadiusDamage (Variables|Default|GetDestructible) 1e+03 (Transformation|GetActorLocation) 1e+02 1e+03 true)
      (Physics|SetSimulatePhysics (Variables|Default|GetDestructible) true)
      (Variables|Default|SetisBroken true)
      (Utilities|FlowControl|Delay 1e+01)
      (Actor|DestroyActor))))

(fn ConstructionScript)