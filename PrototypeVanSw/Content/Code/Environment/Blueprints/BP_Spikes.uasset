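; BP_Spikes is an environmental hazard that damages actors entering or staying inside its sphere trigger.
; On overlap, the player takes base damage only through its capsule component, while any other actor takes a tenfold hit.
; A Tick-accumulated timer periodically applies base damage to every actor still overlapping the sphere.
; All damage is sent as truncated integers through an ApplyDamageMessage call on the affected actor.
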(event OnComponentBeginOverlap(Sphere)
  (params (OverlappedComponent :type Primitive%20Component%20Object%20Reference) (OtherActor :type Actor%20Object%20Reference) (OtherComp :type Primitive%20Component%20Object%20Reference) (OtherBodyIndex :type Integer) (bFromSweep :type Boolean) (SweepResult :type Hit%20Result%20Structure%20%28by%20ref%29))
  (Utilities|Casting|CastToBP_Player OtherActor
    (:then
      (Utilities|Casting|CastToCapsuleComponent OtherComp)
      (Class|BPIonHit|ApplyDamage(Message) OtherActor (Math|Float|Truncate (Variables|Default|GetfDamage))))
    (:CastFailed
      (Class|BPIonHit|ApplyDamage(Message) OtherActor (Math|Float|Truncate (* 10 (Variables|Default|GetfDamage)))))))

(event EventBeginPlay)

(event Collision|EventActorBeginOverlap
  (params (OtherActor :type Actor%20Object%20Reference)))

(event EventTick
  (params (DeltaSeconds :type Float%20%28single-precision%29))
  (bind _output_get (Variables|Default|SetfCurrentTime (+ DeltaSeconds (Variables|Default|GetfCurrentTime))))
  (if (>= _output_get (Variables|Default|GetfTimeBetweenDamageForStaying))
    (Variables|Default|SetfCurrentTime 0.0)
    (for _array_element (Collision|GetOverlappingActors (Variables|Default|GetSphere) "/Script/Engine.Actor" :!class /Script/Engine.PrimitiveComponent)
      (Class|BPIonHit|ApplyDamage(Message) _array_element (Math|Float|Truncate (Variables|Default|GetfDamage))))))

(fn ConstructionScript)