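; BP_DestructiblePillar is an environment pillar that shatters after taking a set number of hits.
; Each ApplyDamage call increments a hit counter until it reaches HitsToBreak, ignoring further calls once broken.
; Breaking applies a large radius damage and impulse to the Destructible component at the actor's location and enables its physics simulation.
; The actor destroys itself ten seconds later.
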(event EventApplyDamage
  (params (DPSBasicAttackDamage :type Integer))
  (if (not (Variables|Default|GetisBroken))
    (bind _output_get (Variables|Default|SetHitsCount (+ (Variables|Default|GetHitsCount) 1.0)))
    (if (>= _output_get (Variables|Default|GetHitsToBreak))
      (Class|DestructibleComponent|ApplyRadiusDamage (Variables|Default|GetDestructible) 2e+04 (Transformation|GetActorLocation) 2e+03 2e+04 true)
      (Physics|SetSimulatePhysics (Variables|Default|GetDestructible) true)
      (Variables|Default|SetisBroken true)
      (Utilities|FlowControl|Delay 1e+01)
      (Actor|DestroyActor))))

(fn ConstructionScript)