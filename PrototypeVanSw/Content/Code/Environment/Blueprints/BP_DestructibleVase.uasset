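; Destructible vase environment actor that shatters after taking a set number of hits.
; Each ApplyDamage event increments a hit counter, ignoring any damage amount, and compares it to HitsToBreak.
; At the threshold, it applies full radius damage with an impulse to its Destructible component at the actor's location and enables physics simulation.
; The actor destroys itself after a short delay.
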(event EventBeginPlay)

(event Collision|EventActorBeginOverlap
  (params (OtherActor :type Actor%20Object%20Reference)))

(event EventTick
  (params (DeltaSeconds :type Float%20%28single-precision%29)))

(event EventApplyDamage
  (params (DPSBasicAttackDamage :type Integer))
  (bind _output_get (Variables|Default|SetHitsCount (+ (Variables|Default|GetHitsCount) 1.0)))
  (if (>= _output_get (Variables|Default|GetHitsToBreak))
    (Class|DestructibleComponent|ApplyRadiusDamage (Variables|Default|GetDestructible) 1e+03 (Transformation|GetActorLocation) 1e+02 1e+03 true)
    (Physics|SetSimulatePhysics (Variables|Default|GetDestructible) true)
    (Utilities|FlowControl|Delay 5.0)
    (Actor|DestroyActor)))

(fn ConstructionScript)