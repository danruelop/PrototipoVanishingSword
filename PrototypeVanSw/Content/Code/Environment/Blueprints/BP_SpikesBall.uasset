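; BP_SpikesBall is a pushable physics spiked ball hazard that damages actors touching its collision.
; On overlap it deals base damage to the player's capsule and heavily multiplied damage to anything else, while Tick re-applies base damage to all overlapping actors at intervals.
; Push applies a scaled impulse to the ball, and Tick keeps the marked component hovering above it as the point GetMarkPoint returns.
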(event OnComponentBeginOverlap(Collision)
  (params (OverlappedComponent :type Primitive%20Component%20Object%20Reference) (OtherActor :type Actor%20Object%20Reference) (OtherComp :type Primitive%20Component%20Object%20Reference) (OtherBodyIndex :type Integer) (bFromSweep :type Boolean) (SweepResult :type Hit%20Result%20Structure%20%28by%20ref%29))
  (Utilities|Casting|CastToBP_Player OtherActor
    (:then
      (Utilities|Casting|CastToCapsuleComponent OtherComp)
      (Class|BPIonHit|ApplyDamage(Message) OtherActor (Math|Float|Truncate (Variables|Default|GetfDamage))))
    (:CastFailed
      ;[1 1 1] Dmg not player
      (Class|BPIonHit|ApplyDamage(Message) OtherActor (Math|Float|Truncate (* 20 (Variables|Default|GetfDamage)))))))

(event EventBeginPlay)

(event Collision|EventActorBeginOverlap
  (params (OtherActor :type Actor%20Object%20Reference)))

(event EventTick
  (params (DeltaSeconds :type Float%20%28single-precision%29))
  (bind _ball (Variables|Default|GetBall))
  (bind _returnvalue (Transformation|GetWorldLocation _ball))
  (Utilities|FlowControl|Sequence
    (:then_0
      (Transformation|SetWorldLocation (Variables|Default|GetBP_C_MarkedComponent) (Math|Vector|MakeVector (.x _returnvalue) (.y _returnvalue) (+ (.z _returnvalue) 4.3e+02)) false false))
    (:then_1
      (bind _output_get (Variables|Default|SetfCurrentTime (+ DeltaSeconds (Variables|Default|GetfCurrentTime))))
      (if (>= _output_get (Variables|Default|GetfTimeBetweenDamageForStaying))
        (Variables|Default|SetfCurrentTime 0.0)
        (for _array_element (Collision|GetOverlappingActors (Variables|Default|GetCollision) "/Script/Engine.Actor" :!class /Script/Engine.PrimitiveComponent)
          (Class|BPIonHit|ApplyDamage(Message) _array_element (Math|Float|Truncate (Variables|Default|GetfDamage))))))))

(event EventPush
  (params (fForceMultiplier :type Float%20%28single-precision%29) (direction :type Vector :default "0, 0, 0"))
  (Physics|AddImpulse (Variables|Default|GetBall) (* direction (* fForceMultiplier 1999988.0)) "None" false))

(fn ConstructionScript)

(fn GetMarkPoint
  (return (Transformation|GetWorldLocation (Variables|Default|GetBP_C_MarkedComponent))))