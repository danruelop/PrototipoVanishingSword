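; Sliceable environment actor that is cut in two when its ApplyDamage event fires.
; The construction script copies the Cube static mesh into a procedural mesh with collision.
; ApplyDamage slices that mesh along a horizontal plane at a fixed height above the actor's origin, capping the cut with CubeMaterial.
; The new half gets physics and an impulse to knock it away, and a sword slice sound plays.
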(event EventBeginPlay)

(event Collision|EventActorBeginOverlap
  (params (OtherActor :type Actor%20Object%20Reference)))

(event EventTick
  (params (DeltaSeconds :type Float%20%28single-precision%29)))

(event EventApplyDamage
  (params (DPSBasicAttackDamage :type Integer))
  (bind _returnvalue (Transformation|GetActorLocation))
  (bind _outotherhalfprocmesh (Class|KismetProceduralMeshLibrary|SliceProceduralMesh (Variables|Default|GetProceduralMesh) (Math|Vector|MakeVector (.x _returnvalue) (.y _returnvalue) (+ (.z _returnvalue) 1e+02)) "0.000000,0.000000,1.000000" true "CreateNewSectionForCap" "/Game/Geometry/Meshes/CubeMaterial.CubeMaterial"))
  (Physics|SetSimulatePhysics _outotherhalfprocmesh true)
  (Physics|AddImpulse _outotherhalfprocmesh "100.000000,100.000000,100.000000" "None" true)
  (Audio|PlaySoundatLocation "/Game/Code/Environment/Sounds/SwordSliceSound.SwordSliceSound" (Transformation|GetActorLocation) "0, 0, 0" 0.25 1.0 0.0 0 0 0))

(fn ConstructionScript
  (Class|KismetProceduralMeshLibrary|CopyProceduralMeshfromStaticMeshComponent (Variables|Default|GetCube) 0 (Variables|Default|GetProceduralMesh) true))